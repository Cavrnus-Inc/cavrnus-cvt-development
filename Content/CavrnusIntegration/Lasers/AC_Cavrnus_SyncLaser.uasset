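; Actor component that syncs a pawn's left or right laser, chosen in the editor, over Cavrnus; setup skips VR pawns.
; After the space connects, it polls for the spawned laser, requesting the spawn first on remote pawns.
; The local owner streams hand, active state, endpoints and color as JSON through transient "LaserBeam" string updates while firing.
; Remote copies parse that property to drive laser visibility, endpoints and color.
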(event Custom|SpaceConnected
  (params (SpaceConnection :type Cavrnus%20Space%20Connection%20Structure))
  (bind _returnvalue (Components|GetOwner))
  ;[0.006856 1 0] Setup - Get specified Laser
  (Variables|Default|SetSpace%20Connection SpaceConnection)
  (Utilities|IsValid _returnvalue
    (:Is%20Valid
      (bind _asbp_base_pawn (Utilities|Casting|CastToBP_BasePawn _returnvalue)
        (:then
          (Utilities|Casting|CastToBP_VRPawn _asbp_base_pawn
            (:CastFailed
              (Utilities|FlowControl|Delay 1.0)
              (bind _output_get (Variables|Default|SetBasePawn _asbp_base_pawn))
              (Variables|Default|SetIsLocalOwner (Pawn|IsLocallyControlled _output_get))
              (Variables|Default|SetContainerName (Variables|/Game/CollaborativeViewer/Blueprints/Pawn/BP_BasePawn.BP_BasePawn_C|GetContainer%20Name (Variables|Default|GetBasePawn)))
              (Utilities|FlowControl|Sequence
                (:then_0
                  (CallFunction|SetupLaser))
                (:then_1
                  (CallFunction|SetupReceiveBindings))
                (:then_2
                  (CallFunction|SetupDestroyLasers))))))
        (:CastFailed
          (Development|PrintString "[AC_Cavrnus_SyncLaser] Failed casting to BP_BasePawn!"))))))

(event Custom|SetupLaser
  (bind _basepawn (Variables|Default|GetBasePawn))
  ;[1 1 1] Get Laser by handedness set in editor
  (if (not (Variables|Default|GetIsLocalOwner))
    (bind _asbp_vrpawn (Utilities|Casting|CastToBP_VRPawn (Variables|Default|GetBasePawn))
      (:then
        ;;[0 0 0] Spawn lasers if user is remote. Wait until lasers are spawned and found
        (Default|SpawnLaseronServer _asbp_vrpawn)
        (bind _foundlaser (Utilities|FindNewlySpawnedLasers _asbp_vrpawn)
          (:Is%20Valid
            (Variables|Default|SetLaser _foundlaser))))
      (:CastFailed
        (Default|SpawnLaseronServer _basepawn)
        (bind _foundlaser_2 (Utilities|FindNewlySpawnedLasers _basepawn)
          (:Is%20Valid
            (Variables|Default|SetLaser _foundlaser_2)))))
    (else
      (bind _asbp_vrpawn_2 (Utilities|Casting|CastToBP_VRPawn (Variables|Default|GetBasePawn))
        (:then
          (bind _foundlaser_3 (Utilities|FindNewlySpawnedLasers _asbp_vrpawn_2)
            (:Is%20Valid
              (Variables|Default|SetLaser _foundlaser_3))))
        (:CastFailed
          (bind _foundlaser_4 (Utilities|FindNewlySpawnedLasers (Variables|Default|GetBasePawn))
            (:Is%20Valid
              (Variables|Default|SetLaser _foundlaser_4)))))))
  (Development|PrintString (Utilities|String|Append "Found: " (select (Variables|Default|GetEditorIsLeftLaser) "Left Laser!" "Right Laser!")) true true "(R=1.000000,G=0.619768,B=0.212178,A=1.000000)" 5.0))

(event Custom|SetupReceiveBindings
  ;[1 1 1] Setup Receive Bindings
  (if (not (Variables|Default|GetIsLocalOwner))
    (Class|CavrnusFunctionLibrary|BindStringPropertyValue (Variables|Default|GetSpace%20Connection) (Variables|Default|GetContainerName) "LaserBeam" (delegate Custom|LaserInfoUpdated))))

(event Custom|LaserInfoUpdated
  (params (Value :type String) (ContainerName :type String) (PropertyName :type String))
  ;[1 1 1] Setup Receive Bindings
  (bind (_outjsonobject _returnvalue) (Class|JsonBlueprintFunctionLibrary|FromString Value))
  (Variables|Default|SetJson%20Object _outjsonobject)
  (if _returnvalue
    (Utilities|FlowControl|Sequence
      (:then_0
        (bind (_outvalue _returnvalue_2) (|GetJsonField (Variables|Default|GetJson%20Object) "Hand"))
        (if _returnvalue_2
          (Variables|ServerValues|SetServerIsLeftHand (Utilities|Enum|Equal(Enum) _outvalue "Left"))))
      (:then_1
        (bind (_outvalue_2 _returnvalue_3) (|GetJsonField (Variables|Default|GetJson%20Object) "Active"))
        (if _returnvalue_3
          (Variables|ServerValues|SetSeverHandActive _outvalue_2)))
      (:then_2
        (bind (_outvalue_3 _returnvalue_4) (|GetJsonField (Variables|Default|GetJson%20Object) "Start"))
        (if _returnvalue_4
          (Variables|ServerValues|SetServerLaserStartPos _outvalue_3)))
      (:then_3
        (bind (_outvalue_4 _returnvalue_5) (|GetJsonField (Variables|Default|GetJson%20Object) "End"))
        (if _returnvalue_5
          (Variables|ServerValues|SetServerLaserEndPos _outvalue_4)))
      (:then_4
        (bind (_outvalue_5 _returnvalue_6) (|GetJsonField (Variables|Default|GetJson%20Object) "Color"))
        (if _returnvalue_6
          (Variables|ServerValues|SetSeverColor _outvalue_5)))
      (:then_5
        (CallFunction|SetLaserVis)))))

(event Custom|Debug
  ;[1 0.58 0.03331] Debug
  (Development|PrintString (Utilities|String|Append "SetString: StartPos=" (Utilities|String|ToString(Vector) (Variables|ServerValues|GetServerLaserStartPos)) " End Pos=" (Utilities|String|ToString(Vector) (Variables|ServerValues|GetServerLaserEndPos)) " Active=" (Utilities|String|ToString(Boolean) (Variables|ServerValues|GetSeverHandActive)))))

(event Custom|SetupDestroyLasers
  (Game|BindEventtoOnDestroyed (Variables|Default|GetBasePawn) (delegate Custom|ActorDestroyed)))

(event Custom|ActorDestroyed
  (params (DestroyedActor :type Actor%20Object%20Reference))
  (Variables|Default|GetBasePawn
    (:then
      (bind _laser (Variables|Default|GetLaser)
        (:then
          (Actor|DestroyActor _laser))
        (:else)))
    (:else)))

(event EventBeginPlay
  ;[0.006856 1 0] Setup - Get specified Laser
  (Class|CavrnusFunctionLibrary|AwaitAnySpaceConnection (delegate Custom|SpaceConnected)))

(event EventTick
  (params (DeltaSeconds :type Float%20%28single-precision%29))
  ;[1 1 1] Transient Laser Updates
  (Variables|Default|GetBasePawn
    (:then
      (Variables|Default|GetLaser
        (:then
          (if (Variables|Default|GetIsLocalOwner)
            (if (select (Variables|Default|GetEditorIsLeftLaser) (Variables|/Game/CollaborativeViewer/Blueprints/Pawn/BP_BasePawn.BP_BasePawn_C|GetIsShootingLaser_L (Variables|Default|GetBasePawn)) (Variables|/Game/CollaborativeViewer/Blueprints/Pawn/BP_BasePawn.BP_BasePawn_C|GetIsShootingLaser_R (Variables|Default|GetBasePawn)))
              (Variables|Default|GetLivePropertyUpdate
                (:then
                  (bind _returnvalue (CallFunction|GetLaserInfo))
                  (Class|CavrnusLiveStringPropertyUpdate|UpdatewithNewData (Variables|Default|GetLivePropertyUpdate) _returnvalue))
                (:else
                  (bind _returnvalue_2 (CallFunction|GetLaserInfo))
                  (bind _returnvalue_3 (Class|CavrnusFunctionLibrary|BeginTransientStringPropertyUpdate (Variables|Default|GetSpace%20Connection) (Variables|Default|GetContainerName) "LaserBeam" _returnvalue_2))
                  (Variables|Default|SetLivePropertyUpdate _returnvalue_3)))
              (else
                (Variables|Default|GetLivePropertyUpdate
                  (:then
                    (bind _returnvalue_4 (CallFunction|GetLaserInfo))
                    (Class|CavrnusLiveStringPropertyUpdate|UpdatewithNewData (Variables|Default|GetLivePropertyUpdate) _returnvalue_4)
                    (Variables|Default|SetLivePropertyUpdate 0))
                  (:else))))))
        (:else)))
    (:else)))

(fn GetLaserInfo
  (Variables|Default|GetLaser
    (:then
      (LocalVariables|SetJsonObject (Utilities|Struct|MakeJsonObjectWrapper))
      (Utilities|FlowControl|Sequence
        (:then_0
          (|SetJsonField (LocalVariables|GetJsonObject) "Hand" (select (Variables|Default|GetEditorIsLeftLaser) "Left" "Right")))
        (:then_1
          (|SetJsonField (LocalVariables|GetJsonObject) "Active" (select (Variables|Default|GetEditorIsLeftLaser) (Variables|/Game/CollaborativeViewer/Blueprints/Pawn/BP_BasePawn.BP_BasePawn_C|GetIsShootingLaser_L (Variables|Default|GetBasePawn)) (Variables|/Game/CollaborativeViewer/Blueprints/Pawn/BP_BasePawn.BP_BasePawn_C|GetIsShootingLaser_R (Variables|Default|GetBasePawn)))))
        (:then_2
          (|SetJsonField (LocalVariables|GetJsonObject) "Start" (Variables|/Game/CollaborativeViewer/Blueprints/Pawn/Laser.Laser_C|GetHitLaserStart (Variables|Default|GetLaser))))
        (:then_3
          (|SetJsonField (LocalVariables|GetJsonObject) "End" (Variables|/Game/CollaborativeViewer/Blueprints/Pawn/Laser.Laser_C|GetHitLaserEnd (Variables|Default|GetLaser))))
        (:then_4
          (|SetJsonField (LocalVariables|GetJsonObject) "Color" (Variables|/Game/CollaborativeViewer/Blueprints/Pawn/BP_BasePawn.BP_BasePawn_C|GetPlayerColor (Variables|Default|GetBasePawn))))
        (:then_5
          ;[1 0.1865 0.1865] Return Value
          (bind _outjsonstring (Class|JsonBlueprintFunctionLibrary|ToString (LocalVariables|GetJsonObject)))
          (return _outjsonstring))))
    (:else)))

(fn SetLaserVis
  (bind _laser (Variables|Default|GetLaser)
    (:then
      (bind _basepawn (Variables|Default|GetBasePawn)
        (:then
          (if (Variables|Default|GetEditorIsLeftLaser)
            (bind _output_get (Variables|/Game/CollaborativeViewer/Blueprints/Pawn/BP_BasePawn.BP_BasePawn_C|SetIsShootingLaser_L _basepawn (Variables|ServerValues|GetSeverHandActive)))
            (Rendering|SetActorHiddenInGame _laser (not _output_get))
            (else
              (bind _output_get_2 (Variables|/Game/CollaborativeViewer/Blueprints/Pawn/BP_BasePawn.BP_BasePawn_C|SetIsShootingLaser_R _basepawn (Variables|ServerValues|GetSeverHandActive)))
              (Rendering|SetActorHiddenInGame _laser (not _output_get_2))))
          (Variables|/Game/CollaborativeViewer/Blueprints/Pawn/Laser.Laser_C|SetHitLaserStart _laser (Variables|ServerValues|GetServerLaserStartPos))
          (Variables|/Game/CollaborativeViewer/Blueprints/Pawn/Laser.Laser_C|SetHitLaserEnd _laser (Variables|ServerValues|GetServerLaserEndPos))
          (Variables|/Game/CollaborativeViewer/Blueprints/Pawn/Laser.Laser_C|SetColor _laser (Variables|ServerValues|GetSeverColor)))
        (:else)))
    (:else)))