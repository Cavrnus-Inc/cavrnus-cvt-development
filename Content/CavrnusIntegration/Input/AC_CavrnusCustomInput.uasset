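; Input component for the Cavrnus pawn that turns rotate-axis and push/pull input into object transform offsets.
; On setup it binds pitch, roll and yaw inputs to pawn flags, keeping RotateMode on while any axis is active.
; With left mouse held and the transform component ticking, mouse wheel values add to its location offset outside rotate mode, or to each active axis's rotation offset.
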(event Custom|Pitch
  (params (Value :type Boolean))
  (bind _pawn (Variables|Default|GetPawn))
  ;[1 1 1] SetupInputLogic
  (bind _pawn_2 (Variables|Default|GetPawn)
    (:then
      (bind _output_get (Variables|/Game/CollaborativeViewer/Blueprints/Pawn/BP_BasePawn.BP_BasePawn_C|SetTransformPitch _pawn_2 Value))
      (if _output_get
        (Variables|/Game/CollaborativeViewer/Blueprints/Pawn/BP_BasePawn.BP_BasePawn_C|SetRotateMode (Variables|Default|GetPawn) true)
        (elif (not (Variables|/Game/CollaborativeViewer/Blueprints/Pawn/BP_BasePawn.BP_BasePawn_C|GetTransformRoll _pawn))
          (if (not (Variables|/Game/CollaborativeViewer/Blueprints/Pawn/BP_BasePawn.BP_BasePawn_C|GetTransformPitch _pawn))
            (if (not (Variables|/Game/CollaborativeViewer/Blueprints/Pawn/BP_BasePawn.BP_BasePawn_C|GetTransformYaw _pawn))
              (Variables|/Game/CollaborativeViewer/Blueprints/Pawn/BP_BasePawn.BP_BasePawn_C|SetRotateMode (Variables|Default|GetPawn) false))))))
    (:else)))

(event Custom|Roll
  (params (Value :type Boolean))
  (bind _pawn (Variables|Default|GetPawn))
  ;[1 1 1] SetupInputLogic
  (bind _pawn_2 (Variables|Default|GetPawn)
    (:then
      (bind _output_get (Variables|/Game/CollaborativeViewer/Blueprints/Pawn/BP_BasePawn.BP_BasePawn_C|SetTransformRoll _pawn_2 Value))
      (if _output_get
        (Variables|/Game/CollaborativeViewer/Blueprints/Pawn/BP_BasePawn.BP_BasePawn_C|SetRotateMode (Variables|Default|GetPawn) true)
        (elif (not (Variables|/Game/CollaborativeViewer/Blueprints/Pawn/BP_BasePawn.BP_BasePawn_C|GetTransformRoll _pawn))
          (if (not (Variables|/Game/CollaborativeViewer/Blueprints/Pawn/BP_BasePawn.BP_BasePawn_C|GetTransformPitch _pawn))
            (if (not (Variables|/Game/CollaborativeViewer/Blueprints/Pawn/BP_BasePawn.BP_BasePawn_C|GetTransformYaw _pawn))
              (Variables|/Game/CollaborativeViewer/Blueprints/Pawn/BP_BasePawn.BP_BasePawn_C|SetRotateMode (Variables|Default|GetPawn) false))))))
    (:else)))

(event Custom|Yaw
  (params (Value :type Boolean))
  (bind _pawn (Variables|Default|GetPawn))
  ;[1 1 1] SetupInputLogic
  (bind _pawn_2 (Variables|Default|GetPawn)
    (:then
      (bind _output_get (Variables|/Game/CollaborativeViewer/Blueprints/Pawn/BP_BasePawn.BP_BasePawn_C|SetTransformYaw _pawn_2 Value))
      (if _output_get
        (Variables|/Game/CollaborativeViewer/Blueprints/Pawn/BP_BasePawn.BP_BasePawn_C|SetRotateMode (Variables|Default|GetPawn) true)
        (elif (not (Variables|/Game/CollaborativeViewer/Blueprints/Pawn/BP_BasePawn.BP_BasePawn_C|GetTransformRoll _pawn))
          (if (not (Variables|/Game/CollaborativeViewer/Blueprints/Pawn/BP_BasePawn.BP_BasePawn_C|GetTransformPitch _pawn))
            (if (not (Variables|/Game/CollaborativeViewer/Blueprints/Pawn/BP_BasePawn.BP_BasePawn_C|GetTransformYaw _pawn))
              (Variables|/Game/CollaborativeViewer/Blueprints/Pawn/BP_BasePawn.BP_BasePawn_C|SetRotateMode (Variables|Default|GetPawn) false))))))
    (:else)))

(event Custom|PushPull
  (params (Value :type Float%20%28double-precision%29))
  (bind _transformcomponent (Variables|Default|GetTransformComponent))
  (bind _pawn (Variables|Default|GetPawn))
  ;[1 1 1] SetupPushAndPull
  (Variables|Default|SetCurrentMouseWheelValue Value)
  (if (Variables|/Game/CollaborativeViewer/Blueprints/Pawn/BP_BasePawn.BP_BasePawn_C|GetIsLeftMousePressed (Variables|Default|GetPawn))
    (if (Class|ActorComponent|IsComponentTickEnabled (Variables|Default|GetTransformComponent))
      (Utilities|FlowControl|Sequence
        (:then_0
          (if (not (Variables|/Game/CollaborativeViewer/Blueprints/Pawn/BP_BasePawn.BP_BasePawn_C|GetRotateMode _pawn))
            (Variables|/Game/CollaborativeViewer/Blueprints/Commands/Transform/BP_TransformComponent.BP_TransformComponent_C|SetActorOffsetLocation_R _transformcomponent (+ (Variables|/Game/CollaborativeViewer/Blueprints/Commands/Transform/BP_TransformComponent.BP_TransformComponent_C|GetActorOffsetLocation_R _transformcomponent) (Variables|Default|GetCurrentMouseWheelValue)))))
        (:then_1
          (if (Variables|/Game/CollaborativeViewer/Blueprints/Pawn/BP_BasePawn.BP_BasePawn_C|GetTransformYaw _pawn)
            (Variables|/Game/CollaborativeViewer/Blueprints/Commands/Transform/BP_TransformComponent.BP_TransformComponent_C|SetCavrnus_OffsetRotationYaw _transformcomponent (+ (Variables|/Game/CollaborativeViewer/Blueprints/Commands/Transform/BP_TransformComponent.BP_TransformComponent_C|GetCavrnus_OffsetRotationYaw _transformcomponent) (Variables|Default|GetCurrentMouseWheelValue)))))
        (:then_2
          (if (Variables|/Game/CollaborativeViewer/Blueprints/Pawn/BP_BasePawn.BP_BasePawn_C|GetTransformRoll _pawn)
            (Variables|/Game/CollaborativeViewer/Blueprints/Commands/Transform/BP_TransformComponent.BP_TransformComponent_C|SetCavrnus_OffsetRotationRoll _transformcomponent (+ (Variables|/Game/CollaborativeViewer/Blueprints/Commands/Transform/BP_TransformComponent.BP_TransformComponent_C|GetCavrnus_OffsetRotationRoll _transformcomponent) (Variables|Default|GetCurrentMouseWheelValue)))))
        (:then_3
          (if (Variables|/Game/CollaborativeViewer/Blueprints/Pawn/BP_BasePawn.BP_BasePawn_C|GetTransformPitch _pawn)
            (Variables|/Game/CollaborativeViewer/Blueprints/Commands/Transform/BP_TransformComponent.BP_TransformComponent_C|SetCavrnus_OffsetRotationPitch _transformcomponent (+ (Variables|/Game/CollaborativeViewer/Blueprints/Commands/Transform/BP_TransformComponent.BP_TransformComponent_C|GetCavrnus_OffsetRotationPitch _transformcomponent) (Variables|Default|GetCurrentMouseWheelValue)))))))))

(event Custom|SetupRotateAxis
  (bind _pawn (Variables|Default|GetPawn))
  ;[1 1 1] SetupInputLogic
  (EventDispatchers|BindEventtoCavrnusPitchInput _pawn (delegate Custom|Pitch))
  (EventDispatchers|BindEventtoCavrnusRollInput _pawn (delegate Custom|Roll))
  (EventDispatchers|BindEventtoCavrnusYawInput _pawn (delegate Custom|Yaw)))

(event Custom|SetupPushPull
  ;[1 1 1] SetupPushAndPull
  (EventDispatchers|BindEventtoCavrnusPushPullInput (Variables|Default|GetPawn) (delegate Custom|PushPull)))

(event EventOnGetComponents
  (bind _pawn (Variables|Default|GetPawn))
  (bind _returnvalue (Actor|GetComponentbyClass _pawn "/Game/CollaborativeViewer/Blueprints/Commands/Transform/BP_TransformComponent.BP_TransformComponent_C"))
  ;[1 0.9636 0.2193] OnGetComponents
  (Utilities|IsValid _returnvalue
    (:Is%20Valid
      (Variables|Default|SetTransformComponent _returnvalue))))

(event EventOnSetupComplete
  ;[0.1454 1 0.1919] OnSetupComplete
  (Utilities|FlowControl|Sequence
    (:then_0
      (CallFunction|SetupRotateAxis))
    (:then_1
      (CallFunction|SetupPushPull))))