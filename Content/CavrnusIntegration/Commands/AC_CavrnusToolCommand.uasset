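; Base actor component for Cavrnus tool commands, providing setup and binding cleanup for its subclasses.
; On BeginPlay it awaits a space connection, caches it with the Collab player controller and base pawn, then subscribes to Cavrnus pawn spawns after a short delay.
; Empty OnGetComponents and OnSetupComplete hooks run on initial setup and each pawn spawn.
; A TrashCan array collects bindings, which are unbound on spawn before the hooks rerun.
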(event Custom|SpaceConnected
  (params (SpaceConnection :type Cavrnus%20Space%20Connection%20Structure))
  (bind _returnvalue (Game|GetPlayerController 0))
  ;[0.1454 1 0.1919] BeginPlay
  (Variables|Cavrnus|SetSpace%20Connection SpaceConnection)
  (Utilities|IsValid _returnvalue
    (:Is%20Valid
      (bind _asbp_collab_v_player_controller (Utilities|Casting|CastToBP_Collab_V_PlayerController _returnvalue)
        (:then
          (Variables|CVT|SetPlayerController _asbp_collab_v_player_controller)
          (bind _asbp_base_pawn (Utilities|Casting|CastToBP_BasePawn (Game|Player|GetPlayerPawn 0))
            (:then
              (Variables|CVT|SetPawn _asbp_base_pawn)
              (Utilities|FlowControl|Delay 0.2)
              (Utilities|FlowControl|Sequence
                (:then_0
                  (CallFunction|BindtoPawnSpawn))
                (:then_1
                  (CallFunction|OnGetComponents))
                (:then_2
                  (CallFunction|OnSetupComplete))))
            (:CastFailed
              (Development|PrintString "AC_CavrnusToolCommand: Cannot find local Pawn"))))
        (:CastFailed
          (Development|PrintString "AC_CavrnusToolCommand: Cannot find player controller!"))))))

(event Custom|OnSetupComplete
  ;[0.1454 1 0.1919] BeginPlay
)

(event Custom|OnGetComponents
  ;[0.1454 1 0.1919] BeginPlay
)

(event Custom|BindToPawnSpawn
  ;[1 0.9636 0.2193] BindToPawnSpawn
  (EventDispatchers|BindEventtoCavrnusPawnSpawned (Variables|CVT|GetPlayerController) (delegate Custom|OnPawnSpawned)))

(event Custom|OnPawnSpawned
  ;[1 0.9636 0.2193] BindToPawnSpawn
  (Utilities|FlowControl|Sequence
    (:then_0
      (CallFunction|EmptyTrashCan))
    (:then_1
      (CallFunction|OnGetComponents))
    (:then_2
      (CallFunction|OnSetupComplete))))

(event Custom|EmptyTrashCan
  ;[1 0 0.1002] TrashCan
  (for _array_element (Variables|Cavrnus|GetTrashCan)
    (Utilities|IsValid _array_element
      (:Is%20Valid
        (Class|CavrnusBinding|Unbind _array_element))))
  (Utilities|Array|Clear (Variables|Cavrnus|GetTrashCan)))

(event EventBeginPlay
  ;[0.1454 1 0.1919] BeginPlay
  (Class|CavrnusFunctionLibrary|AwaitAnySpaceConnection (delegate Custom|SpaceConnected)))

(fn AddtoTrashCan
  (params (Binding :type Cavrnus%20Binding%20Object%20Reference))
  (Utilities|Array|Add (Variables|Cavrnus|GetTrashCan) Binding))