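; Actor component that networks crop box creation through Cavrnus spaces.
; It finds the pawn's crop box component and binds to its spawn-loader event after setup.
; When that event fires, it spawns a shared crop box loader object in the space.
; It then posts the gizmo transform at the given location and initial interaction and inclusion flags as synced properties.
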(event Custom|SetupBindings
  ;[1 1 1] SetupBindings
  (EventDispatchers|BindEventtoCavrnusSpawnCropBoxLoader (Variables|Default|GetCropboxComponent) (delegate Custom|CustomEvent)))

(event Custom|CustomEvent
  (params (Location :type Transform))
  ;[1 1 1] SetupBindings
  (bind _returnvalue (Class|CavrnusFunctionLibrary|SpawnObject (Variables|Default|GetSpace%20Connection) "BP_Cavrnus_CropboxLoader"))
  (Class|CavrnusFunctionLibrary|PostTransformPropertyUpdate (.spaceconnection _returnvalue) (.propertiescontainername _returnvalue) "Gizmo" Location)
  (Class|CavrnusFunctionLibrary|PostBoolPropertyUpdate (.spaceconnection _returnvalue) (.propertiescontainername _returnvalue) "IsInteracting" false)
  (Class|CavrnusFunctionLibrary|PostBoolPropertyUpdate (.spaceconnection _returnvalue) (.propertiescontainername _returnvalue) "IsIncluding" false))

(event EventOnGetComponents
  (bind _pawn (Variables|Default|GetPawn))
  (bind _returnvalue (Actor|GetComponentbyClass _pawn "/Game/CollaborativeViewer/Blueprints/Commands/CropBox/BP_CropBoxComponent.BP_CropBoxComponent_C"))
  ;[1 0.9636 0.2193] OnGetComponents
  (Utilities|IsValid _returnvalue
    (:Is%20Valid
      (Variables|Default|SetCropboxComponent _returnvalue))))

(event EventOnSetupComplete
  ;[0.1454 1 0.1919] OnSetupComplete
  (Variables|Default|GetCropboxComponent
    (:then
      (Utilities|FlowControl|Sequence
        (:then_0
          (CallFunction|SetupBindings))))
    (:else)))