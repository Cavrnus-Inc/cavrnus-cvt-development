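; Cavrnus loader actor that spawns a BP_CropBox and keeps it synced across a shared space.
; On space connection it spawns the box at the stored "Gizmo" transform, then attaches a properties container and gizmo sync component.
; Include/exclude and interaction states post to and update from bound boolean properties.
; Destruction links both ways: losing the box destroys the spawned space object, and losing the loader destroys the box.
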(event Custom|OnSpaceConnected
  (params (SpaceConnection :type Cavrnus%20Space%20Connection%20Structure))
  (bind _returnvalue (Actor|GetComponentbyClass "/Script/CavrnusConnector.CavrnusPropertiesContainer"))
  (Variables|Default|SetSpaceConnection SpaceConnection)
  (Utilities|FlowControl|Delay 0.0)
  (Utilities|IsValid _returnvalue
    (:Is%20Valid
      (bind _output_get (Variables|Default|SetContainerName (Variables|/Script/CavrnusConnector.CavrnusPropertiesContainer|GetContainerName _returnvalue)))
      (bind _returnvalue_2 (Class|CavrnusFunctionLibrary|GetTransformPropertyValue (Variables|Default|GetSpaceConnection) _output_get "Gizmo"))
      (bind _returnvalue_3 (Game|SpawnActorfromClass "/Game/CollaborativeViewer/Blueprints/Commands/CropBox/BPs/BP_CropBox.BP_CropBox_C" _returnvalue_2 "Undefined" "OverrideRootScale" 0 0 0))
      (Variables|Default|SetCropBox _returnvalue_3)
      (Utilities|FlowControl|Sequence
        (:then_0
          (CallFunction|SetuponDestroy))
        (:then_1
          (CallFunction|AddSyncCropBoxLocation))
        (:then_2
          (CallFunction|SetupBindings))))))

(event Custom|SetupBindings
  ;[1 1 1] SetupBindings
  (EventDispatchers|BindEventtoCavrnusSetExcludeInclude (Variables|Default|GetCropBox) (delegate Custom|IncludeExcludeChanged))
  (Class|CavrnusFunctionLibrary|BindBooleanPropertyValue (Variables|Default|GetSpaceConnection) (Variables|Default|GetContainerName) "IsIncluding" (delegate Custom|IsIncludeUpdated))
  (EventDispatchers|BindEventtoCavrnusSetInteractionState (Variables|Default|GetCropBox) (delegate Custom|InteractingChanged))
  (Class|CavrnusFunctionLibrary|BindBooleanPropertyValue (Variables|Default|GetSpaceConnection) (Variables|Default|GetContainerName) "IsInteracting" (delegate Custom|IsInteractUpdated)))

(event Custom|AddSyncCropBoxLocation
  (bind _cropbox (Variables|Default|GetCropBox))
  ;[1 1 1] Add Sync Location
  (bind _returnvalue (AddComponent|AddCavrnusPropertiesContainer (Variables|Default|GetCropBox) true))
  (Variables|/Script/CavrnusConnector.CavrnusPropertiesContainer|SetContainerName _returnvalue (Variables|Default|GetContainerName))
  (Game|AddComponentbyClass :self _cropbox :Class "/Game/CavrnusIntegration/Commands/CropBox/AC_SyncCropBoxGizmo.AC_SyncCropBoxGizmo_C" :bManualAttachment true :CropBox _cropbox :PropertyName "Gizmo"))

(event Custom|OnDestroyedEvent
  (params (DestroyedActor :type Actor%20Object%20Reference))
  (bind _returnvalue (Actor|GetComponentbyClass "/Script/CavrnusConnector.CavrnusSpawnedObjectFlag"))
  ;[1 1 1] Setup OnDestroy
  (Utilities|IsValid _returnvalue
    (:Is%20Valid
      (Class|CavrnusFunctionLibrary|DestroyObject (Variables|/Script/CavrnusConnector.CavrnusSpawnedObjectFlag|GetSpawnedObject _returnvalue)))))

(event Custom|IsInteractUpdated
  (params (Value :type Boolean) (ContainerName :type String) (PropertyName :type String))
  ;[1 1 1] SetupBindings
  (Variables|/Game/CollaborativeViewer/Blueprints/Commands/CropBox/BPs/BP_CropBox.BP_CropBox_C|SetInteracting (Variables|Default|GetCropBox) Value))

(event Custom|IncludeExcludeChanged
  (params (IsInclude :type Boolean))
  ;[1 1 1] SetupBindings
  (Class|CavrnusFunctionLibrary|PostBoolPropertyUpdate (Variables|Default|GetSpaceConnection) (Variables|Default|GetContainerName) "IsIncluding" IsInclude))

(event Custom|IsIncludeUpdated
  (params (Value :type Boolean) (ContainerName :type String) (PropertyName :type String))
  (bind _cropbox (Variables|Default|GetCropBox))
  ;[1 1 1] SetupBindings
  (bind _output_get (Variables|/Game/CollaborativeViewer/Blueprints/Commands/CropBox/BPs/BP_CropBox.BP_CropBox_C|SetisInclude (Variables|Default|GetCropBox) Value))
  (if _output_get
    (Default|HideActorsIncludeModeMTC _cropbox)
    (else
      (Default|ShowAllActorHiden _cropbox))))

(event Custom|DestroyedRemotely
  (params (DestroyedActor :type Actor%20Object%20Reference))
  ;[1 1 1] Setup OnDestroy
  (bind _cropbox (Variables|Default|GetCropBox)
    (:then
      (Actor|DestroyActor _cropbox))
    (:else)))

(event Custom|SetupOnDestroy
  ;[1 1 1] Setup OnDestroy
  (Game|AssignOnDestroyed (Variables|Default|GetCropBox) (delegate Custom|OnDestroyedEvent))
  (Game|BindEventtoOnDestroyed (delegate Custom|DestroyedRemotely)))

(event Custom|InitializePawnReference
  ;[1 1 1] Initialize Pawn Reference.
  (bind _asbp_base_pawn (Utilities|Casting|CastToBP_BasePawn (Game|Player|GetPlayerPawn 0)))
  (Variables|/Game/CollaborativeViewer/Blueprints/Commands/CropBox/BPs/BP_CropBox.BP_CropBox_C|SetPawnInteracting (Variables|Default|GetCropBox) _asbp_base_pawn))

(event Custom|InteractingChanged
  (params (IsInteracting :type Boolean))
  ;[1 1 1] SetupBindings
  (Class|CavrnusFunctionLibrary|PostBoolPropertyUpdate (Variables|Default|GetSpaceConnection) (Variables|Default|GetContainerName) "IsInteracting" IsInteracting))

(event EventBeginPlay
  (Class|CavrnusFunctionLibrary|AwaitAnySpaceConnection (delegate Custom|OnSpaceConnected)))

(fn ConstructionScript)