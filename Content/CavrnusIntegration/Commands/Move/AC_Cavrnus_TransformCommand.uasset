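; Cavrnus command component that shares actor move, reset and reset-all actions across a space through the pawn's BP_TransformComponent.
; Local modifications post as JSON actor-tag lists to "ModifiedTransforms" string properties: Move persists, while resets are immediately cancelled transient updates that also prune the Move list.
; Incoming Move updates attach properties containers and relative-transform sync components to tagged actors lacking world sync, then update TransformManager.
; Incoming resets restore transforms through the transform component.
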(event Custom|Modified
  (params (ActionType :type String) (ModfiedActors :type Array%20of%20Strings))
  ;[1 1 1] Setup Bindings
  (CallFunction|ProcessModifiedTransforms ActionType ModfiedActors))

(event Custom|Updated
  (params (Value :type String) (ContainerName :type String) (PropertyName :type String))
  ;[1 1 1] Setup Bindings
  (if (not (Utilities|Array|IsEmpty Value))
    (bind (_actors _success) (CallFunction|GetModifiedActorsArray Value))
    (if _success
      (CallFunction|ActionMove _actors))))

(event Custom|Reset
  (params (Value :type String) (ContainerName :type String) (PropertyName :type String))
  ;[1 1 1] Setup Bindings
  (if (not (Utilities|Array|IsEmpty Value))
    (bind (_actors _success) (CallFunction|GetModifiedActorsArray Value))
    (if _success
      (CallFunction|ActionReset _actors))))

(event Custom|ResetAll
  (params (Value :type String) (ContainerName :type String) (PropertyName :type String))
  ;[1 1 1] Setup Bindings
  (if (not (Utilities|Array|IsEmpty Value))
    (bind (_actors _success) (CallFunction|GetModifiedActorsArray Value))
    (if _success
      (CallFunction|ActionResetAll _actors))))

(event Custom|SetupBindings
  ;[1 1 1] Setup Bindings
  (EventDispatchers|BindEventtoCavrnusModifiedActorsEvent (Variables|Default|GetTransformComponent) (delegate Custom|Modified))
  (bind _returnvalue (Class|CavrnusFunctionLibrary|BindStringPropertyValue (Variables|Default|GetSpace%20Connection) "ModifiedTransforms" "Move" (delegate Custom|Updated)))
  (CallFunction|AddtoTrashCan _returnvalue)
  (bind _returnvalue_2 (Class|CavrnusFunctionLibrary|BindStringPropertyValue (Variables|Default|GetSpace%20Connection) "ModifiedTransforms" "Reset" (delegate Custom|Reset)))
  (CallFunction|AddtoTrashCan _returnvalue_2)
  (bind _returnvalue_3 (Class|CavrnusFunctionLibrary|BindStringPropertyValue (Variables|Default|GetSpace%20Connection) "ModifiedTransforms" "ResetAll" (delegate Custom|ResetAll)))
  (CallFunction|AddtoTrashCan _returnvalue_3))

(event Custom|ActionMove
  (params (Actors :type Array%20of%20Strings))
  ;[1 1 1] Move
  (bind _transformmanager (Variables|Default|GetTransformManager)
    (:then
      (for _array_element Actors
        (if (.ActorFound (CallFunction|GetActorfromTag _array_element))
          (Utilities|IsValid (.Actor (CallFunction|GetActorfromTag _array_element))
            (:Is%20Valid
              (Utilities|IsValid (Actor|GetComponentbyClass (.Actor (CallFunction|GetActorfromTag _array_element)) "/CavrnusConnector/SamplePropertySynchronizers/AC_SyncWorldTransform.AC_SyncWorldTransform_C")
                (:Is%20Not%20Valid
                  (bind _returnvalue (Game|AddComponentbyClass (.Actor (CallFunction|GetActorfromTag _array_element)) "/Script/CavrnusConnector.CavrnusPropertiesContainer" true))
                  (Variables|/Script/CavrnusConnector.CavrnusPropertiesContainer|SetContainerName _returnvalue _array_element)
                  (Game|AddComponentbyClass (.Actor (CallFunction|GetActorfromTag _array_element)) "/CavrnusConnector/SamplePropertySynchronizers/AC_SyncRelativeTransform.AC_SyncRelativeTransform_C" true)))))))
      (Variables|/Game/CollaborativeViewer/Blueprints/Commands/Transform/BPs/TransformManager.TransformManager_C|SetTransformedActors _transformmanager Actors))
    (:else)))

(event Custom|ActionReset
  (params (Actors :type Array%20of%20Strings))
  ;[1 1 1] Reset
  (for _array_element Actors
    (Default|RestoreInitialTransformRunOnserver (Variables|Default|GetTransformComponent) _array_element)))

(event Custom|ActionResetAll
  (params (Actors :type Array%20of%20Strings))
  ;[1 1 1] RestoreAll
  (Variables|/Game/CollaborativeViewer/Blueprints/Commands/Transform/BPs/TransformManager.TransformManager_C|SetTransformedActors (Variables|Default|GetTransformManager) Actors)
  (Default|RestoreTransformAll (Variables|Default|GetTransformComponent)))

(event EventOnGetComponents
  (bind _pawn (Variables|Default|GetPawn))
  (bind _returnvalue (Actor|GetComponentbyClass _pawn "/Game/CollaborativeViewer/Blueprints/Commands/Transform/BP_TransformComponent.BP_TransformComponent_C"))
  ;[1 0.9636 0.2193] GetComponents
  (Utilities|IsValid _returnvalue
    (:Is%20Valid
      (bind _output_get (Variables|Default|SetTransformComponent _returnvalue))
      (Variables|Default|SetTransformManager (Variables|/Game/CollaborativeViewer/Blueprints/Commands/Transform/BP_TransformComponent.BP_TransformComponent_C|GetTransformManager _output_get)))))

(event EventOnSetupComplete
  ;[0.1454 1 0.1919] SetupComplete
  (CallFunction|SetupBindings))

(fn PostAction
  (params (ActionType :type String) (ModifiedTransforms :type Array%20of%20Strings))
  (bind _jsonobjectwrapper (Utilities|Struct|MakeJsonObjectWrapper))
  (|SetJsonField _jsonobjectwrapper ActionType ModifiedTransforms)
  (bind _outjsonstring (Class|JsonBlueprintFunctionLibrary|ToString _jsonobjectwrapper))
  (switch string ActionType
    (:Move
      (Class|CavrnusFunctionLibrary|PostStringPropertyUpdate (Variables|Default|GetSpace%20Connection) "ModifiedTransforms" "Move" _outjsonstring))
    (:Reset
      (bind _returnvalue (Class|CavrnusFunctionLibrary|BeginTransientStringPropertyUpdate (Variables|Default|GetSpace%20Connection) "ModifiedTransforms" "Reset" _outjsonstring))
      (Class|CavrnusLivePropertyUpdate|Cancel _returnvalue))
    (:ResetAll
      (bind _returnvalue_2 (Class|CavrnusFunctionLibrary|BeginTransientStringPropertyUpdate (Variables|Default|GetSpace%20Connection) "ModifiedTransforms" "ResetAll" _outjsonstring))
      (Class|CavrnusLivePropertyUpdate|Cancel _returnvalue_2))))

(fn GetModifiedActorsArray
  (params (InJsonString :type String))
  (bind (_outjsonobject _returnvalue) (Class|JsonBlueprintFunctionLibrary|FromString InJsonString))
  (if _returnvalue
    (bind (_fieldnames _returnvalue_2) (Class|JsonBlueprintFunctionLibrary|GetFieldNames _outjsonobject))
    (if _returnvalue_2
      (bind (_outvalue _returnvalue_3) (|GetJsonField _outjsonobject (Utilities|Array|Get(acopy) _fieldnames)))
      (if _returnvalue_3
        _
        (else
          _))
      (return _outvalue _returnvalue_3)
      (else
        (return 0 _returnvalue_2)))
    (else
      (return 0 _returnvalue))))

(fn GetActionType
  (params (InJsonString :type String))
  (bind (_outjsonobject _returnvalue) (Class|JsonBlueprintFunctionLibrary|FromString InJsonString))
  (if _returnvalue
    (bind (_fieldnames _returnvalue_2) (Class|JsonBlueprintFunctionLibrary|GetFieldNames _outjsonobject))
    (if _returnvalue_2
      (return (Utilities|Array|Get(acopy) _fieldnames)))))

(fn ProcessModifiedTransforms
  (params (ActionType :type String) (Actors :type Array%20of%20Strings))
  (Utilities|Array|Clear (LocalVariables|GetTempArray))
  (switch string ActionType
    (:Move
      (CallFunction|PostAction ActionType Actors))
    (:Reset
      (bind _modifiedactors (CallFunction|GetModifedMoveTransforms Actors))
      (CallFunction|PostAction "Move" _modifiedactors)
      (CallFunction|PostAction "Reset" Actors))
    (:ResetAll
      (bind _modifiedactors_2 (CallFunction|GetModifedMoveTransforms Actors))
      (CallFunction|PostAction "Move" _modifiedactors_2)
      (CallFunction|PostAction "ResetAll" Actors))))

(fn GetModifedMoveTransforms
  (params (Actors :type Array%20of%20Strings))
  (Utilities|Array|AppendArray (LocalVariables|GetTempArray) (Variables|/Game/CollaborativeViewer/Blueprints/Commands/Transform/BPs/TransformManager.TransformManager_C|GetTransformedActors (Variables|Default|GetTransformManager)))
  (for _array_element Actors
    (Utilities|Array|RemoveItem (LocalVariables|GetTempArray) _array_element))
  (return (LocalVariables|GetTempArray)))