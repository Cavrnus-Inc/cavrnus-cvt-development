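; Actor component that shares the owner's record of moved actors through a Cavrnus space.
; On connection, after a short delay, it takes the TransformManager from the owner's BP_TransformComponent and seeds TransformedActors from a stored JSON string property.
; It then posts the manager's modified-actor updates back to that property as JSON.
; Remote changes are only read at startup, and the component-level update binding is never executed.
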(event Custom|SpaceConnected
  (params (SpaceConnection :type Cavrnus%20Space%20Connection%20Structure))
  (bind _returnvalue (Components|GetOwner))
  (bind _returnvalue_2 (Actor|GetComponentbyClass _returnvalue "/Game/CollaborativeViewer/Blueprints/Commands/Transform/BP_TransformComponent.BP_TransformComponent_C"))
  (Variables|Default|SetSpace%20Connection SpaceConnection)
  (Utilities|FlowControl|Delay 0.2)
  (Utilities|IsValid _returnvalue
    (:Is%20Valid
      (Utilities|IsValid _returnvalue_2
        (:Is%20Valid
          (bind _output_get (Variables|Default|SetTransformComponent _returnvalue_2))
          (Variables|Default|SetTransformManager (Variables|/Game/CollaborativeViewer/Blueprints/Commands/Transform/BP_TransformComponent.BP_TransformComponent_C|GetTransformManager _output_get))
          (Utilities|FlowControl|Sequence
            (:then_0
              (CallFunction|InitializeModifiedObjects))
            (:then_1
              (CallFunction|SetupBindings))))))))

(event Custom|InitializeModifiedObjects
  ;[1 1 1] Initialize Modified Objects
  (bind (_outjsonobject _returnvalue) (CallFunction|GetServerObjects))
  (if _returnvalue
    (bind (_outvalue _returnvalue_2) (|GetJsonField _outjsonobject "TransformActors"))
    (if _returnvalue_2
      (bind _transformmanager (Variables|Default|GetTransformManager)
        (:then
          (Variables|/Game/CollaborativeViewer/Blueprints/Commands/Transform/BPs/TransformManager.TransformManager_C|SetTransformedActors _transformmanager _outvalue))
        (:else))
      (else
        (Development|PrintString "AC_Cavrnus_SyncMove: Unable to GetField(TransformActor)")))))

(event Custom|SetupBindings
  ;[1 1 1] Setup Bindings
  (bind _transformmanager (Variables|Default|GetTransformManager)
    (:then
      (EventDispatchers|BindEventtoCavrnusModifiedActorsEvent _transformmanager (delegate Custom|ManagerUpdated)))
    (:else)))

(event Custom|ComponentUpdated
  (params (ModfiedActors :type Array%20of%20Strings))
  ;[1 1 1] Setup Bindings
  (CallFunction|PostModifiedTransforms ModfiedActors))

(event Custom|ManagerUpdated
  (params (ModifiedActors :type Array%20of%20Strings))
  ;[1 1 1] Setup Bindings
  (CallFunction|PostModifiedTransforms ModifiedActors))

(event EventBeginPlay
  (Class|CavrnusFunctionLibrary|AwaitAnySpaceConnection (delegate Custom|SpaceConnected)))

(fn GetServerObjects
  (bind _returnvalue (Class|CavrnusFunctionLibrary|GetStringPropertyValue (Variables|Default|GetSpace%20Connection) "TransformActors" "Modified"))
  (bind (_outjsonobject _returnvalue_2) (Class|JsonBlueprintFunctionLibrary|FromString _returnvalue))
  (return _outjsonobject _returnvalue_2))

(fn PostModifiedTransforms
  (params (ModifiedTransforms :type Array%20of%20Strings))
  (bind _jsonobjectwrapper (Utilities|Struct|MakeJsonObjectWrapper))
  (|SetJsonField _jsonobjectwrapper "TransformActors" ModifiedTransforms)
  (bind _outjsonstring (Class|JsonBlueprintFunctionLibrary|ToString _jsonobjectwrapper))
  (Class|CavrnusFunctionLibrary|PostStringPropertyUpdate (Variables|Default|GetSpace%20Connection) "TransformActors" "Modified" _outjsonstring))