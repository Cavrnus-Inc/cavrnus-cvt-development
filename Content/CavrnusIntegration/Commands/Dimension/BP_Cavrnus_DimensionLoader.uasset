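; Cavrnus loader actor that spawns a local BP_Dimenssion measurement actor and keeps it in sync with space properties.
; On space connection it reads its properties container name, spawns the dimension, and binds endpoints, location, update-once flag and units to it.
; Destruction is linked both ways: destroying the dimension destroys the Cavrnus spawned object, and destroying the loader destroys the dimension.
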(event Custom|SpaceConnected
  (params (SpaceConnection :type Cavrnus%20Space%20Connection%20Structure))
  (bind _returnvalue (Actor|GetComponentbyClass "/Script/CavrnusConnector.CavrnusPropertiesContainer"))
  (Variables|Default|SetSpace%20Connection SpaceConnection)
  (Utilities|FlowControl|Delay 0.0)
  (Utilities|IsValid _returnvalue
    (:Is%20Valid
      (Variables|Default|SetContainer%20Name (Variables|/Script/CavrnusConnector.CavrnusPropertiesContainer|GetContainerName _returnvalue))
      (bind _returnvalue_2 (Game|SpawnActorfromClass "/Game/CollaborativeViewer/Blueprints/Commands/Dimension/BPs/BP_Dimenssion.BP_Dimenssion_C" (Math|Transform|MakeTransform "0, 0, 0") "Undefined" "OverrideRootScale" 0 "0.000000,0.000000,0.000000" "0.000000,0.000000,100.000000" 0 "NewEnumerator1" true 0))
      (bind _output_get (Variables|Default|SetDimension _returnvalue_2))
      (Utilities|IsValid _output_get
        (:Is%20Valid
          (Utilities|FlowControl|Sequence
            (:then_0
              (CallFunction|SetupDestroy))
            (:then_1
              (CallFunction|SetupBindings))))))))

(event Custom|SetupBindings
  ;[1 1 1] Setup Bindings
  (Class|CavrnusFunctionLibrary|BindVectorPropertyValue (Variables|Default|GetSpace%20Connection) (Variables|Default|GetContainer%20Name) "PointA" (delegate Custom|LocationAUpdated))
  (Class|CavrnusFunctionLibrary|BindVectorPropertyValue (Variables|Default|GetSpace%20Connection) (Variables|Default|GetContainer%20Name) "PointB" (delegate Custom|LocationBUpdated))
  (Class|CavrnusFunctionLibrary|BindVectorPropertyValue (Variables|Default|GetSpace%20Connection) (Variables|Default|GetContainer%20Name) "Location" (delegate Custom|Location))
  (Class|CavrnusFunctionLibrary|BindBooleanPropertyValue (Variables|Default|GetSpace%20Connection) (Variables|Default|GetContainer%20Name) "UpdateOnce" (delegate Custom|UpdateOnce))
  (Class|CavrnusFunctionLibrary|BindStringPropertyValue (Variables|Default|GetSpace%20Connection) (Variables|Default|GetContainer%20Name) "Units" (delegate Custom|UnitsUpdated)))

(event Custom|UnitsUpdated
  (params (Value :type String) (ContainerName :type String) (PropertyName :type String))
  (bind _dimension (Variables|Default|GetDimension))
  ;[1 1 1] Setup Bindings
  (Variables|Default|GetDimension
    (:then
      (switch string Value
        (:Default
          (Variables|/Game/CollaborativeViewer/Blueprints/Commands/Dimension/BPs/BP_Dimenssion.BP_Dimenssion_C|SetUnits _dimension "NewEnumerator1" :!label _label))
        (:Meter
          (goto _label))
        (:Centimeter
          (Variables|/Game/CollaborativeViewer/Blueprints/Commands/Dimension/BPs/BP_Dimenssion.BP_Dimenssion_C|SetUnits _dimension "NewEnumerator0"))
        (:Imperial
          (Variables|/Game/CollaborativeViewer/Blueprints/Commands/Dimension/BPs/BP_Dimenssion.BP_Dimenssion_C|SetUnits _dimension "NewEnumerator2"))))
    (:else)))

(event Custom|SetupDestroy
  ;[1 1 1] Setup Destroy
  (Game|BindEventtoOnDestroyed (Variables|Default|GetDimension) (delegate Custom|Destroyed))
  (Game|BindEventtoOnDestroyed (delegate Custom|DestroyedRemotely)))

(event Custom|Destroyed
  (params (DestroyedActor :type Actor%20Object%20Reference))
  (bind _returnvalue (Actor|GetComponentbyClass "/Script/CavrnusConnector.CavrnusSpawnedObjectFlag"))
  ;[1 1 1] Setup Destroy
  (Utilities|IsValid _returnvalue
    (:Is%20Valid
      (Class|CavrnusFunctionLibrary|DestroyObject (Variables|/Script/CavrnusConnector.CavrnusSpawnedObjectFlag|GetSpawnedObject _returnvalue)))))

(event Custom|DestroyedRemotely
  (params (DestroyedActor :type Actor%20Object%20Reference))
  ;[1 1 1] Setup Destroy
  (bind _dimension (Variables|Default|GetDimension)
    (:then
      (Actor|DestroyActor _dimension))
    (:else)))

(event Custom|LocationAUpdated
  (params (Value :type Vector%204%20Structure) (ContainerName :type String) (PropertyName :type String))
  ;[1 1 1] Setup Bindings
  (bind _dimension (Variables|Default|GetDimension)
    (:then
      (Variables|/Game/CollaborativeViewer/Blueprints/Commands/Dimension/BPs/BP_Dimenssion.BP_Dimenssion_C|SetPointA _dimension (Math|Conversions|ToVector(Vector4) Value)))
    (:else)))

(event Custom|LocationBUpdated
  (params (Value :type Vector%204%20Structure) (ContainerName :type String) (PropertyName :type String))
  ;[1 1 1] Setup Bindings
  (bind _dimension (Variables|Default|GetDimension)
    (:then
      (Variables|/Game/CollaborativeViewer/Blueprints/Commands/Dimension/BPs/BP_Dimenssion.BP_Dimenssion_C|SetPointB _dimension (Math|Conversions|ToVector(Vector4) Value)))
    (:else)))

(event Custom|Location
  (params (Value :type Vector%204%20Structure) (ContainerName :type String) (PropertyName :type String))
  (bind (_x _y _z) (Math|Vector4|BreakVector4 Value))
  ;[1 1 1] Setup Bindings
  (bind _dimension (Variables|Default|GetDimension)
    (:then
      (Transformation|SetActorTransform _dimension (Math|Transform|MakeTransform (Math|Vector|MakeVector _x _y _z) "0, 0, 0" "1.000000,1.000000,1.000000")))
    (:else)))

(event Custom|UpdateOnce
  (params (Value :type Boolean) (ContainerName :type String) (PropertyName :type String))
  ;[1 1 1] Setup Bindings
  (bind _dimension (Variables|Default|GetDimension)
    (:then
      (Variables|/Game/CollaborativeViewer/Blueprints/Commands/Dimension/BPs/BP_Dimenssion.BP_Dimenssion_C|SetUpdateOnce _dimension Value))
    (:else)))

(event EventBeginPlay
  (Class|CavrnusFunctionLibrary|AwaitAnySpaceConnection (delegate Custom|SpaceConnected)))

(fn ConstructionScript)