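; Actor component command that replicates dimensions created on the pawn into a Cavrnus space as shared objects.
; It finds the pawn's BP_DimensionComponent and, on setup completion, binds to its dimension-created event.
; Each event spawns a BP_Cavrnus_DimensionLoader object through the space connection, then posts endpoints, location, units and the update-once flag to that object's properties container.
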(event Custom|SetupBinding
  ;[1 1 1] SetupBinding
  (EventDispatchers|BindEventtoCavrnusDimensionCreated (Variables|Default|GetDimensionComponent) (delegate Custom|CreateDimension)))

(event Custom|CreateDimension
  (params (PointA :type Vector) (PointB :type Vector) (Location :type Vector) (Units :type String) (UpdateOnce :type Boolean))
  (bind (_x _y _z) (Math|Vector|BreakVector PointA))
  (bind (_x_2 _y_2 _z_2) (Math|Vector|BreakVector PointB))
  (bind _space_connection (Variables|Default|GetSpace%20Connection))
  ;[1 1 1] SetupBinding
  (bind _returnvalue (Class|CavrnusFunctionLibrary|SpawnObject (Variables|Default|GetSpace%20Connection) "BP_Cavrnus_DimensionLoader"))
  (Utilities|FlowControl|Sequence
    (:then_0
      (Class|CavrnusFunctionLibrary|PostVectorPropertyUpdate _space_connection (.propertiescontainername _returnvalue) "PointA" (Math|Vector4|MakeVector4 _x _y _z 0.0)))
    (:then_1
      (Class|CavrnusFunctionLibrary|PostVectorPropertyUpdate _space_connection (.propertiescontainername _returnvalue) "PointB" (Math|Vector4|MakeVector4 _x_2 _y_2 _z_2 0.0)))
    (:then_2
      (Class|CavrnusFunctionLibrary|PostVectorPropertyUpdate _space_connection (.propertiescontainername _returnvalue) "Location" (Math|Vector4|MakeVector4 (.x Location) (.y Location) (.z Location) 0.0)))
    (:then_3
      (Class|CavrnusFunctionLibrary|PostStringPropertyUpdate _space_connection (.propertiescontainername _returnvalue) "Units" Units))
    (:then_4
      (Class|CavrnusFunctionLibrary|PostBoolPropertyUpdate _space_connection (.propertiescontainername _returnvalue) "UpdateOnce" UpdateOnce))))

(event EventOnSetupComplete
  ;[0.1454 1 0.1919] SetupComplete
  (Variables|Default|GetDimensionComponent
    (:then
      (Utilities|FlowControl|Sequence
        (:then_0
          (CallFunction|SetupBinding))))
    (:else)))

(event EventOnGetComponents
  ;[1 0.9636 0.2193] OnGetComponents
  (Variables|Default|SetDimensionComponent (Actor|GetComponentbyClass (Variables|Default|GetPawn) "/Game/CollaborativeViewer/Blueprints/Commands/Dimension/BP_DimensionComponent.BP_DimensionComponent_C")))