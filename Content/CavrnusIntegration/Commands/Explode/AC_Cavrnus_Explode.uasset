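; Actor component that syncs exploded-view animations on a BP_BasePawn owner over a Cavrnus space connection.
; Once connected, it finds the pawn's BP_ExplodeComponent and binds a boolean "Active" property per ExplodeData entry, with containers keyed by name and index.
; Property updates set the explode flag and a target transform, then start the animation, reading element and index directly from the binding loop's outputs.
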(event Custom|SpaceConnected
  (params (SpaceConnection :type Cavrnus%20Space%20Connection%20Structure))
  (Variables|Default|SetSpace%20Connection SpaceConnection)
  (Utilities|FlowControl|Delay 0.0)
  (bind _asbp_base_pawn (Utilities|Casting|CastToBP_BasePawn (Components|GetOwner))
    (:then
      (bind _output_get (Variables|Default|SetAs%20BP%20Base%20Pawn _asbp_base_pawn))
      (Variables|Default|SetExplode (Actor|GetComponentbyClass _output_get "/Game/CollaborativeViewer/Blueprints/Commands/Explode/BP_ExplodeComponent.BP_ExplodeComponent_C"))
      (Utilities|FlowControl|Sequence
        (:then_0
          (CallFunction|SetupBindings))))
    (:CastFailed
      (Development|PrintString "Failed casting to BP_BasePawn: AC_Cavrnus_Explode must be on BasePawn!"))))

(event Custom|SetupBindings
  ;[1 1 1] Setup Bindings to react to selection
  (for (_array_element _array_index) (Variables|/Game/CollaborativeViewer/Blueprints/Commands/Explode/BP_ExplodeComponent.BP_ExplodeComponent_C|GetExplodeData (Variables|Default|GetExplode))
    (Class|CavrnusFunctionLibrary|BindBooleanPropertyValue (Variables|Default|GetSpace%20Connection) (Utilities|String|Append "ExplodeObject" (Utilities|GetDisplayName _array_element) (Utilities|String|ToString(Integer) _array_index)) "Active" (delegate Custom|AnimationUpdated))))

(event Custom|AnimationUpdated
  (params (Value :type Boolean) (ContainerName :type String) (PropertyName :type String))
  ;[1 1 1] Setup Bindings to react to selection
  (bind _output_get (Variables|/Game/CollaborativeViewer/Blueprints/Commands/Explode/BP_Explode.BP_Explode_C|SetIsExplode (stale Custom|SetupBindings _array_element) Value))
  (if _output_get
    (Variables|/Game/CollaborativeViewer/Blueprints/Commands/Explode/BP_Explode.BP_Explode_C|SetCurrentSecondTransform (stale Custom|SetupBindings _array_element) (Variables|/Game/CollaborativeViewer/Blueprints/Commands/Explode/BP_Explode.BP_Explode_C|GetExplodeTransform (stale Custom|SetupBindings _array_element)))
    (else
      (Variables|/Game/CollaborativeViewer/Blueprints/Commands/Explode/BP_Explode.BP_Explode_C|SetCurrentFirstTransform (stale Custom|SetupBindings _array_element) (Variables|/Game/CollaborativeViewer/Blueprints/Commands/Explode/BP_Explode.BP_Explode_C|GetInitialTransform (stale Custom|SetupBindings _array_element)))))
  (Default|StartAnimMTC (Variables|Default|GetExplode) (stale Custom|SetupBindings _array_index)))

(event EventBeginPlay
  (Class|CavrnusFunctionLibrary|AwaitAnySpaceConnection (delegate Custom|SpaceConnected)))