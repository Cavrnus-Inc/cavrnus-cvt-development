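; Actor component that syncs exploded-view toggles from the pawn's BP_ExplodeComponent across a Cavrnus space.
; A local toggle reads that entry's server state and posts its inverse as a JSON Id/Active string, using one "ExplodeTool" property per ExplodeData entry.
; Bindings on those properties parse each update, set the entry's explode flag and target transform, then start the animation, so playback is driven by the shared state.
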(event Custom|Triggered
  (params (Input :type Integer))
  ;[1 1 1] Setup Bindings to react to selection
  (CallFunction|PostToggleExplodeAnimation Input (not (CallFunction|GetServerActiveStatefromLocal Input))))

(event Custom|CreateComponentBinding
  ;[1 1 1] Setup Bindings to react to selection
  (EventDispatchers|BindEventtoCavrnusExplodeToggled (Variables|Default|GetExplodeComponent) (delegate Custom|Triggered)))

(event Custom|ValueUpdated
  (params (Value :type String) (ContainerName :type String) (PropertyName :type String))
  ;[1 1 1] CreateBindings
  (CallFunction|HandleExplodeAction (CallFunction|GetExplosionIdfromJson Value) (CallFunction|GetExplosionActivefromJson Value)))

(event Custom|CreateBindings
  ;[1 1 1] CreateBindings
  (for (_ _array_index) (Variables|/Game/CollaborativeViewer/Blueprints/Commands/Explode/BP_ExplodeComponent.BP_ExplodeComponent_C|GetExplodeData (Variables|Default|GetExplodeComponent))
    (bind _returnvalue (Class|CavrnusFunctionLibrary|BindStringPropertyValue (Variables|Default|GetSpace%20Connection) "ExplodeTool" (CallFunction|GetExplosionNamefromLocal _array_index) (delegate Custom|ValueUpdated)))
    (CallFunction|AddtoBindTracker _returnvalue)))

(event Custom|HandleExplodeAction
  (params (Id :type Integer) (State :type Boolean))
  (bind _explodecomponent (Variables|Default|GetExplodeComponent))
  (bind _explodedata (Variables|/Game/CollaborativeViewer/Blueprints/Commands/Explode/BP_ExplodeComponent.BP_ExplodeComponent_C|GetExplodeData _explodecomponent))
  (bind _output (Utilities|Array|Get(acopy) _explodedata Id))
  ;[1 1 1] HandleExplosion
  (Utilities|IsValid _output
    (:Is%20Valid
      (bind _output_get (Variables|/Game/CollaborativeViewer/Blueprints/Commands/Explode/BP_Explode.BP_Explode_C|SetIsExplode _output State))
      (if _output_get
        (Variables|/Game/CollaborativeViewer/Blueprints/Commands/Explode/BP_Explode.BP_Explode_C|SetCurrentSecondTransform _output (Variables|/Game/CollaborativeViewer/Blueprints/Commands/Explode/BP_Explode.BP_Explode_C|GetExplodeTransform _output))
        (else
          (Variables|/Game/CollaborativeViewer/Blueprints/Commands/Explode/BP_Explode.BP_Explode_C|SetCurrentFirstTransform _output (Variables|/Game/CollaborativeViewer/Blueprints/Commands/Explode/BP_Explode.BP_Explode_C|GetInitialTransform _output))))
      (Default|StartAnimROS (Variables|Default|GetExplodeComponent) Id))))

(event EventOnSetupComplete
  ;[0.1454 1 0.1919] SetupComplete
  (Variables|Default|GetExplodeComponent
    (:then
      (Utilities|FlowControl|Sequence
        (:then_0
          (CallFunction|CreateBindings))
        (:then_1
          (CallFunction|CreateComponentBinding))))
    (:else)))

(event EventOnGetComponents
  ;[1 0.9636 0.2193] OnGetComponents
  (Variables|Default|SetExplodeComponent (Actor|GetComponentbyClass (Variables|Default|GetPawn) "/Game/CollaborativeViewer/Blueprints/Commands/Explode/BP_ExplodeComponent.BP_ExplodeComponent_C")))

(fn PostToggleExplodeAnimation
  (params (Id :type Integer) (Active :type Boolean))
  (bind _jsonobjectwrapper (Utilities|Struct|MakeJsonObjectWrapper))
  (|SetJsonField _jsonobjectwrapper "Id" Id)
  (|SetJsonField _jsonobjectwrapper "Active" Active)
  (bind _outjsonstring (Class|JsonBlueprintFunctionLibrary|ToString _jsonobjectwrapper))
  (Class|CavrnusFunctionLibrary|PostStringPropertyUpdate (Variables|Default|GetSpace%20Connection) "ExplodeTool" (CallFunction|GetExplosionNamefromLocal Id) _outjsonstring))

(fn GetServerActiveStatefromLocal
  (params (Id :type Integer))
  (bind _returnvalue (Class|CavrnusFunctionLibrary|GetStringPropertyValue (Variables|Default|GetSpace%20Connection) "ExplodeTool" (CallFunction|GetExplosionNamefromLocal Id)))
  (return (CallFunction|GetExplosionActivefromJson _returnvalue)))

(fn GetExplosionNamefromLocal
  (params (Id :type Integer))
  (return (Utilities|String|Append (Utilities|GetDisplayName (Utilities|Array|Get(acopy) (Variables|/Game/CollaborativeViewer/Blueprints/Commands/Explode/BP_ExplodeComponent.BP_ExplodeComponent_C|GetExplodeData (Variables|Default|GetExplodeComponent)) Id)) (Utilities|String|ToString(Integer) Id))))

(fn GetExplosionIdfromJson
  (params (ServerJson :type String))
  (bind _outjsonobject (Class|JsonBlueprintFunctionLibrary|FromString ServerJson))
  (bind _outvalue (|GetJsonField _outjsonobject "Id"))
  (return _outvalue))

(fn GetExplosionActivefromJson
  (params (ServerJson :type String))
  (bind _outjsonobject (Class|JsonBlueprintFunctionLibrary|FromString ServerJson))
  (bind _outvalue (|GetJsonField _outjsonobject "Active"))
  (return _outvalue))