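; Cavrnus-networked loader actor that rebuilds a shared annotation stroke from synced space properties.
; On space connection it binds its container's transform, color, hand and JSON point-array properties.
; Each update calls UpdateStroke, which, when points exist, destroys and respawns a local BP_Annotation_Stroke at the first point.
; Destroy bindings link both lifetimes: loader destruction removes the stroke, and stroke destruction handlers request deletion of the networked spawned object.
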(event Custom|OnTransformUpdated
  (params (Value :type Transform) (ContainerName :type String) (PropertyName :type String))
  ;[1 1 1] Setup Bindings
  (Variables|Default|SetStartTransform Value)
  (CallFunction|UpdateStroke))

(event Custom|LocallyDestroyed
  (params (DestroyedActor :type Actor%20Object%20Reference))
  ;[1 1 1] Setup Bindings
  (Class|CavrnusFunctionLibrary|DestroyObject (Variables|Default|GetSpawnedObjectFlag)))

(event Custom|SetupBinds
  ;[1 1 1] Setup Bindings
  (Class|CavrnusFunctionLibrary|BindTransformPropertyValue (Variables|Default|GetSpace%20Connection) (Variables|Default|GetContainer%20Name) "Transform" (delegate Custom|OnTransformUpdated))
  (Class|CavrnusFunctionLibrary|BindColorPropertyValue (Variables|Default|GetSpace%20Connection) (Variables|Default|GetContainer%20Name) "Color" (delegate Custom|OnColorUpdated))
  (Class|CavrnusFunctionLibrary|BindBooleanPropertyValue (Variables|Default|GetSpace%20Connection) (Variables|Default|GetContainer%20Name) "IsRightHand" (delegate Custom|IsRightHandUpdated))
  (Class|CavrnusFunctionLibrary|BindStringPropertyValue (Variables|Default|GetSpace%20Connection) (Variables|Default|GetContainer%20Name) "AnnotationTransforms" (delegate Custom|OnTransformsUpdated))
  (Game|BindEventtoOnDestroyed (delegate Custom|RemotelyDeleted))
  (Game|BindEventtoOnDestroyed (Variables|Default|GetNetworkStroke) (delegate Custom|LocallyDestroyed)))

(event Custom|OnColorUpdated
  (params (Value :type Linear%20Color%20Structure) (ContainerName :type String) (PropertyName :type String))
  ;[1 1 1] Setup Bindings
  (Variables|Default|SetColor Value)
  (CallFunction|UpdateStroke))

(event Custom|IsRightHandUpdated
  (params (Value :type Boolean) (ContainerName :type String) (PropertyName :type String))
  ;[1 1 1] Setup Bindings
  (Variables|Default|SetIsRightHand Value)
  (CallFunction|UpdateStroke))

(event Custom|RemotelyDeleted
  (params (DestroyedActor :type Actor%20Object%20Reference))
  ;[1 1 1] Setup Bindings
  (bind _networkstroke (Variables|Default|GetNetworkStroke)
    (:then
      (Actor|DestroyActor _networkstroke))
    (:else)))

(event Custom|OnTransformsUpdated
  (params (Value :type String) (ContainerName :type String) (PropertyName :type String))
  ;[1 1 1] Setup Bindings
  (bind _returnvalue (Class|CvtUtilities|JsonStringtoFTransformArray Value "Transforms"))
  (Variables|Default|SetAnnotationTransforms _returnvalue)
  (CallFunction|UpdateStroke))

(event Custom|SpaceConnected
  (params (SpaceConnection :type Cavrnus%20Space%20Connection%20Structure))
  (bind _returnvalue (Actor|GetComponentbyClass "/Script/CavrnusConnector.CavrnusPropertiesContainer"))
  (Variables|Default|SetSpace%20Connection SpaceConnection)
  (Utilities|FlowControl|Delay 0.0)
  (Utilities|IsValid _returnvalue
    (:Is%20Valid
      (Variables|Default|SetContainer%20Name (Variables|/Script/CavrnusConnector.CavrnusPropertiesContainer|GetContainerName _returnvalue))
      (Variables|Default|SetSpawnedObjectFlag (Variables|/Script/CavrnusConnector.CavrnusSpawnedObjectFlag|GetSpawnedObject (Actor|GetComponentbyClass "/Script/CavrnusConnector.CavrnusSpawnedObjectFlag")))
      (CallFunction|SetupBinds))))

(event EventBeginPlay
  (Class|CavrnusFunctionLibrary|AwaitAnySpaceConnection (delegate Custom|SpaceConnected)))

(fn ConstructionScript)

(fn UpdateStroke
  (bind _annotationtransforms (Variables|Default|GetAnnotationTransforms))
  (if (Utilities|Array|IsNotEmpty (Variables|Default|GetAnnotationTransforms))
    (Utilities|IsValid (Variables|Default|GetNetworkStroke)
      (:Is%20Valid
        (EventDispatchers|UnbindallEventsfromOnDestroyed (Variables|Default|GetNetworkStroke))
        (Actor|DestroyActor (Variables|Default|GetNetworkStroke)))
      (:Is%20Not%20Valid
        _))
    (bind _returnvalue (Game|SpawnActorfromClass "/Game/CollaborativeViewer/Blueprints/Commands/Annotation/BPs/BP_Annotation_Stroke.BP_Annotation_Stroke_C" (Math|Transform|MakeTransform (.Location (Math|Transform|BreakTransform (Utilities|Array|Get(acopy) _annotationtransforms))) "0, 0, 0" "1.000000,1.000000,1.000000") "AlwaysSpawn" 0 _annotationtransforms (Variables|Default|GetColor) true (Variables|Default|GetIsRightHand) false 0))
    (bind _output_get (Variables|Default|SetNetworkStroke _returnvalue))
    (Game|BindEventtoOnDestroyed _output_get (EventDispatchers|CreateEvent :!event OnDestroy))))

(fn OnDestroy
  (params (DestroyedActor :type Actor%20Object%20Reference))
  (bind _networkstroke (Variables|Default|GetNetworkStroke)
    (:then
      (Utilities|IsValid (Actor|GetComponentbyClass _networkstroke "/Script/CavrnusConnector.CavrnusSpawnedObjectFlag")
        (:Is%20Valid
          (Class|CavrnusFunctionLibrary|DestroyObject (Variables|/Script/CavrnusConnector.CavrnusSpawnedObjectFlag|GetSpawnedObject (Actor|GetComponentbyClass _networkstroke "/Script/CavrnusConnector.CavrnusSpawnedObjectFlag"))))))
    (:else)))