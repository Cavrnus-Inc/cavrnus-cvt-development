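; Cavrnus command component that shares a pawn's paint and text annotations in the connected space.
; It binds to the BP_AnnotationComponent's creation events, then spawns a stroke or text loader object and posts its data as Cavrnus properties.
; Stroke transforms are serialized into a JSON string property.
; Each paint stroke also posts a timestamped, user-named bookmark at the camera's transform through the owner's bookmark command.
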(event Custom|TextCreated
  (params (SpawnLocation :type Vector) (Text :type Text) (TextManipulatorRelativeLocation :type Vector))
  ;[1 1 1] SetupComponent
  (CallFunction|PostAnnotationText SpawnLocation Text TextManipulatorRelativeLocation))

(event Custom|SetupComponent
  ;[1 1 1] SetupComponent
  (EventDispatchers|BindEventtoCavrnusPaintCreated (Variables|Default|GetAnnotationComponent) (delegate Custom|PaintCreated))
  (EventDispatchers|BindEventtoCavrnusTextCreated (Variables|Default|GetAnnotationComponent) (delegate Custom|TextCreated)))

(event Custom|PaintCreated
  (params (Transforms :type Array%20of%20Transforms) (StrokeColor :type Linear%20Color%20Structure) (IsRightHand :type Boolean))
  (bind _playercontroller (Variables|Default|GetPlayerController))
  (bind _playercameramanager (Variables|/Script/Engine.PlayerController|GetPlayerCameraManager _playercontroller))
  ;[1 1 1] SetupComponent
  (CallFunction|PostPaintStroke Transforms StrokeColor IsRightHand)
  (bind _returnvalue (Class|CavrnusFunctionLibrary|GetStringPropertyValue (Variables|Default|GetSpace%20Connection) (Variables|Default|GetPawnContainerName) "name"))
  (Default|PostBookmark (Variables|Default|GetCavrnusBookmarkManager) (Utilities|Text|ToText(String) (Utilities|String|Append "Paint: " _returnvalue " " "[" (CallFunction|GetCurrentTime) "]")) (Math|Transform|MakeTransform (Camera|GetCameraLocation _playercameramanager) (Camera|GetCameraRotation _playercameramanager))))

(event EventOnGetComponents
  (bind _returnvalue (Components|GetOwner))
  (bind _pawn (Variables|Default|GetPawn))
  (bind _returnvalue_2 (Actor|GetComponentbyClass _returnvalue "/Game/CavrnusIntegration/Commands/Bookmarks/AC_Cavrnus_BookmarkCommand.AC_Cavrnus_BookmarkCommand_C"))
  (bind _returnvalue_3 (Actor|GetComponentbyClass _pawn "/Game/CollaborativeViewer/Blueprints/Commands/Annotation/BP_AnnotationComponent.BP_AnnotationComponent_C"))
  ;[1 0.9636 0.2193] OnGetComponents
  (Utilities|IsValid _returnvalue_3
    (:Is%20Valid
      (Variables|Default|SetAnnotationComponent _returnvalue_3)
      (Utilities|IsValid _returnvalue_2
        (:Is%20Valid
          (Variables|Default|SetCavrnusBookmarkManager _returnvalue_2))))))

(event EventOnSetupComplete
  ;[0.1454 1 0.1919] SetupComplete
  (CallFunction|SetupComponent))

(fn PostPaintStroke
  (params (Transforms :type Array%20of%20Transforms) (StrokeColor :type Linear%20Color%20Structure) (IsRightHand :type Boolean))
  (bind _jsonobjectwrapper (Utilities|Struct|MakeJsonObjectWrapper))
  (bind _annotationcomponent (Variables|Default|GetAnnotationComponent))
  (LocalVariables|SetCurrentStroke (select IsRightHand (Variables|/Game/CollaborativeViewer/Blueprints/Commands/Annotation/BP_AnnotationComponent.BP_AnnotationComponent_C|GetCurrentStrokeR _annotationcomponent) (Variables|/Game/CollaborativeViewer/Blueprints/Commands/Annotation/BP_AnnotationComponent.BP_AnnotationComponent_C|GetCurrentStrokeL _annotationcomponent)))
  (bind _returnvalue (Class|CavrnusFunctionLibrary|SpawnObject (Variables|Default|GetSpace%20Connection) "BP_Cavrnus_AnnotationLoaderStroke"))
  (Class|CavrnusFunctionLibrary|PostTransformPropertyUpdate (Variables|Default|GetSpace%20Connection) (.PropertiesContainerName (Utilities|Struct|BreakCavrnusSpawnedObject _returnvalue)) "Transform" (Variables|/Game/CollaborativeViewer/Blueprints/Commands/Annotation/BP_AnnotationComponent.BP_AnnotationComponent_C|GetStartTransform (Variables|Default|GetAnnotationComponent)))
  (Class|CavrnusFunctionLibrary|PostColorPropertyUpdate (Variables|Default|GetSpace%20Connection) (.PropertiesContainerName (Utilities|Struct|BreakCavrnusSpawnedObject _returnvalue)) "Color" StrokeColor)
  (Class|CavrnusFunctionLibrary|PostBoolPropertyUpdate (Variables|Default|GetSpace%20Connection) (.PropertiesContainerName (Utilities|Struct|BreakCavrnusSpawnedObject _returnvalue)) "IsRightHand" IsRightHand)
  (|SetJsonField _jsonobjectwrapper "Transforms" Transforms)
  (bind _outjsonstring (Class|JsonBlueprintFunctionLibrary|ToString _jsonobjectwrapper))
  (Class|CavrnusFunctionLibrary|PostStringPropertyUpdate (Variables|Default|GetSpace%20Connection) (.PropertiesContainerName (Utilities|Struct|BreakCavrnusSpawnedObject _returnvalue)) "AnnotationTransforms" _outjsonstring))

(fn PostAnnotationText
  (params (SpawnLocation :type Vector) (Text :type Text) (TextManipulatorRelativeLocation :type Vector))
  (bind _propertypostoptions (Utilities|Struct|MakePropertyPostOptions false))
  (bind _space_connection (Variables|Default|GetSpace%20Connection))
  (bind _returnvalue (Class|CavrnusFunctionLibrary|SpawnObject (Variables|Default|GetSpace%20Connection) "BP_Cavrnus_AnnotationLoaderText"))
  (Utilities|FlowControl|Sequence
    (:then_0
      (Class|CavrnusFunctionLibrary|PostStringPropertyUpdate _space_connection (.propertiescontainername _returnvalue) "AnnotationText" (Utilities|String|ToString(Text) Text)))
    (:then_1
      (Class|CavrnusFunctionLibrary|PostTransformPropertyUpdate _space_connection (.propertiescontainername _returnvalue) "TargetRootTransform" (Math|Conversions|ToTransform(Vector) SpawnLocation) _propertypostoptions))
    (:then_2
      (Class|CavrnusFunctionLibrary|PostTransformPropertyUpdate _space_connection (.propertiescontainername _returnvalue) "TextRootTransform" (Math|Conversions|ToTransform(Vector) TextManipulatorRelativeLocation) _propertypostoptions))))

(fn GetCurrentTime
  (bind _returnvalue (Math|DateTime|Now))
  (bind (_year _month _day _hour _minute) (Math|DateTime|BreakDateTime _returnvalue))
  (Utilities|FlowControl|Sequence
    (:then_0
      (if (== _hour 0)
        (LocalVariables|SetHour "12")
        (elif (> _hour 12)
          (LocalVariables|SetHour (Utilities|String|ToString(Integer) (- _hour 12)))
          (else
            (LocalVariables|SetHour (Utilities|String|ToString(Integer) _hour)))))
      (return (Utilities|String|Append (Utilities|String|ToString(Integer) _month) "/" (Utilities|String|ToString(Integer) _day) "-" (LocalVariables|GetHour) ":" (select (< _minute 10) (Utilities|String|Append "0" (Utilities|String|ToString(Integer) _minute)) (Utilities|String|ToString(Integer) _minute)) (select (< _hour 12) "AM" "PM"))))))