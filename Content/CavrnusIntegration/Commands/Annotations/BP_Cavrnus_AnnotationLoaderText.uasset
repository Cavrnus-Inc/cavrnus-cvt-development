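; Networked loader actor for Cavrnus text annotations that spawns a local BP_AnnotationText once a space connects.
; It binds text and target/text root transform properties from its properties container to that actor, and posts committed text edits back to the space.
; Deletion is linked both ways: destroying the local text destroys the Cavrnus spawned object, and destroying the loader removes the text actor.
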(event Custom|SpaceConnected
  (params (SpaceConnection :type Cavrnus%20Space%20Connection%20Structure))
  (bind _returnvalue (Actor|GetComponentbyClass "/Script/CavrnusConnector.CavrnusPropertiesContainer"))
  (Variables|Default|SetSpace%20Connection SpaceConnection)
  (Utilities|FlowControl|Delay 0.0)
  (Utilities|IsValid _returnvalue
    (:Is%20Valid
      (Variables|Default|SetContainer%20Name (Variables|/Script/CavrnusConnector.CavrnusPropertiesContainer|GetContainerName _returnvalue))
      (bind _returnvalue_2 (Game|SpawnActorfromClass "/Game/CollaborativeViewer/Blueprints/Commands/Annotation/BPs/BP_AnnotationText.BP_AnnotationText_C" (Math|Transform|MakeTransform "0, 0, 0") "Undefined" 0 "" "0.000000,0.000000,0.000000" 0))
      (Variables|Default|SetAnnotateText _returnvalue_2)
      (Utilities|IsValid _returnvalue_2
        (:Is%20Valid
          (Utilities|FlowControl|Sequence
            (:then_0
              (CallFunction|SetuponDestroy))
            (:then_1
              (CallFunction|SetupBinds))))))))

(event Custom|TargetRootUpdated
  (params (Value :type Transform) (ContainerName :type String) (PropertyName :type String))
  ;[1 1 1] Setup Bindings
  (bind _annotatetext (Variables|Default|GetAnnotateText)
    (:then
      (Utilities|IsValid (Variables|/Game/CollaborativeViewer/Blueprints/Commands/Annotation/BPs/BP_AnnotationText.BP_AnnotationText_C|GetTargetRoot _annotatetext)
        (:Is%20Valid
          (Transformation|SetRelativeTransform (Variables|/Game/CollaborativeViewer/Blueprints/Commands/Annotation/BPs/BP_AnnotationText.BP_AnnotationText_C|GetTargetRoot _annotatetext) Value false false))))
    (:else)))

(event Custom|Destroyed
  (params (DestroyedActor :type Actor%20Object%20Reference))
  (bind _returnvalue (Actor|GetComponentbyClass "/Script/CavrnusConnector.CavrnusSpawnedObjectFlag"))
  ;[1 1 1] Setup OnDestroy
  (Utilities|IsValid _returnvalue
    (:Is%20Valid
      (Class|CavrnusFunctionLibrary|DestroyObject (Variables|/Script/CavrnusConnector.CavrnusSpawnedObjectFlag|GetSpawnedObject _returnvalue)))))

(event Custom|TextRootUpdated
  (params (Value :type Transform) (ContainerName :type String) (PropertyName :type String))
  ;[1 1 1] Setup Bindings
  (bind _annotatetext (Variables|Default|GetAnnotateText)
    (:then
      (Utilities|IsValid (Variables|/Game/CollaborativeViewer/Blueprints/Commands/Annotation/BPs/BP_AnnotationText.BP_AnnotationText_C|GetTextRoot _annotatetext)
        (:Is%20Valid
          (Transformation|SetRelativeTransform (Variables|/Game/CollaborativeViewer/Blueprints/Commands/Annotation/BPs/BP_AnnotationText.BP_AnnotationText_C|GetTextRoot _annotatetext) Value false false))))
    (:else)))

(event Custom|SetupOnDestroy
  ;[1 1 1] Setup OnDestroy
  (Game|BindEventtoOnDestroyed (Variables|Default|GetAnnotateText) (delegate Custom|Destroyed))
  (Game|BindEventtoOnDestroyed (delegate Custom|RemotelyDeleted)))

(event Custom|SetupBinds
  ;[1 1 1] Setup Bindings
  (EventDispatchers|BindEventtoOnTextCommitted (Variables|/Game/CollaborativeViewer/Blueprints/Commands/Annotation/UMG/TextAnnotate.TextAnnotate_C|GetAnnotationText (Variables|/Game/CollaborativeViewer/Blueprints/Commands/Annotation/BPs/BP_AnnotationText.BP_AnnotationText_C|Get2DWidget (Variables|Default|GetAnnotateText))) (delegate Custom|TextCommitted))
  (Class|CavrnusFunctionLibrary|BindStringPropertyValue (Variables|Default|GetSpace%20Connection) (Variables|Default|GetContainer%20Name) "AnnotationText" (delegate Custom|TextUpdated))
  (Class|CavrnusFunctionLibrary|BindTransformPropertyValue (Variables|Default|GetSpace%20Connection) (Variables|Default|GetContainer%20Name) "TargetRootTransform" (delegate Custom|TargetRootUpdated))
  (Class|CavrnusFunctionLibrary|BindTransformPropertyValue (Variables|Default|GetSpace%20Connection) (Variables|Default|GetContainer%20Name) "TextRootTransform" (delegate Custom|TextRootUpdated)))

(event Custom|TextUpdated
  (params (Value :type String) (ContainerName :type String) (PropertyName :type String))
  ;[1 1 1] Setup Bindings
  (bind _annotatetext (Variables|Default|GetAnnotateText)
    (:then
      (Variables|Default|SetAnnotateText _annotatetext)
      (Default|SetWidgetText _annotatetext (Utilities|Text|ToText(String) Value)))
    (:else)))

(event Custom|TextCommitted
  (params (Text :type Text%20%28by%20ref%29) (CommitMethod :type ETextCommit%20Enum :default "Default"))
  ;[1 1 1] Setup Bindings
  (Class|CavrnusFunctionLibrary|PostStringPropertyUpdate (Variables|Default|GetSpace%20Connection) (Variables|Default|GetContainer%20Name) "AnnotationText" (Utilities|String|ToString(Text) Text)))

(event Custom|RemotelyDeleted
  (params (DestroyedActor :type Actor%20Object%20Reference))
  ;[1 1 1] Setup OnDestroy
  (bind _annotatetext (Variables|Default|GetAnnotateText)
    (:then
      (Actor|DestroyActor _annotatetext))
    (:else)))

(event EventBeginPlay
  (Class|CavrnusFunctionLibrary|AwaitAnySpaceConnection (delegate Custom|SpaceConnected)))

(fn ConstructionScript)