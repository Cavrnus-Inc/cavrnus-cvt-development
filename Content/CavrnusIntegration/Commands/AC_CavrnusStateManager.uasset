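; Actor component that syncs the current named save state across a Cavrnus space and shares save files through it.
; Saves made in the persistent UI post their slot name to the "State/Current" property, whose binding updates the main save and load-state combo box.
; UploadSaveFile polls for the .sav, spawns a loader object, uploads the file and posts its ID and name there.
; JSON helpers for save, dimension and X-ray data are largely unfinished.
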(event Custom|UploadSaveFile
  (params (Name :type String))
  ;[1 1 1] UploadSaveFile
  (bind _output_get (Variables|Default|SetTargetPath (Utilities|String|TrimTrailing (Utilities|String|Append (Class|FilePaths|GetSavedFolder "SaveGames/") (Utilities|String|TrimTrailing Name) ".sav"))))
  (if (Class|BlueprintPathsLibrary|FileExists _output_get) :!label _label
    (bind _returnvalue (Class|CavrnusFunctionLibrary|SpawnObject (Variables|Default|GetSpace%20Connection) "BP_Cavrnus_SavedGameLoader"))
    (Class|CavrnusFunctionLibrary|UploadContent (Variables|Default|GetTargetPath) (delegate Custom|FileUpload))
    (else
      (Utilities|FlowControl|Delay 0.2)
      (goto _label))))

(event Custom|FileUpload
  (params (uploadedContent :type Cavrnus%20Remote%20Content%20Structure%20%28by%20ref%29))
  (bind (_id _name _filename) (Utilities|Struct|BreakCavrnusRemoteContent uploadedContent))
  (bind _jsonobjectwrapper (Utilities|Struct|MakeJsonObjectWrapper))
  ;[1 1 1] UploadSaveFile
  (Development|PrintString (Utilities|String|Append "Uploaded: " _filename) true true "(R=0.000000,G=0.219293,B=1.000000,A=1.000000)" 2e+01)
  (|SetJsonField _jsonobjectwrapper "Id" _id)
  (|SetJsonField _jsonobjectwrapper "Name" _filename)
  (bind (_outjsonstring _returnvalue) (Class|JsonBlueprintFunctionLibrary|ToString _jsonobjectwrapper))
  (if _returnvalue
    (Class|CavrnusFunctionLibrary|PostStringPropertyUpdate (Variables|Default|GetSpace%20Connection) (.propertiescontainername (stale Custom|UploadSaveFile _returnvalue)) "SaveFile" _outjsonstring)))

(event Custom|SetupBindings
  ;[1 1 1] SetupBindings
  (EventDispatchers|BindEventtoSavingState (Variables|/Game/CollaborativeViewer/Blueprints/PlayerController/BP_Collab_V_PlayerController.BP_Collab_V_PlayerController_C|GetPersistent_UI (Variables|Default|GetPlayerController)) (delegate Custom|SaveGameCreated))
  (Class|CavrnusFunctionLibrary|DefineStringPropertyDefaultValue (Variables|Default|GetSpace%20Connection) "State" "Current" "Default State")
  (Class|CavrnusFunctionLibrary|BindStringPropertyValue (Variables|Default|GetSpace%20Connection) "State" "Current" (delegate Custom|StateChanged)))

(event Custom|SaveGameCreated
  (params (SlotName :type String%20%28by%20ref%29))
  ;[1 1 1] SetupBindings
  (Class|CavrnusFunctionLibrary|PostStringPropertyUpdate (Variables|Default|GetSpace%20Connection) "State" "Current" SlotName))

(event Custom|StateChanged
  (params (Value :type String) (ContainerName :type String) (PropertyName :type String))
  ;[1 1 1] SetupBindings
  (if (not (Utilities|Array|IsEmpty Value))
    (bind _playercontroller (Variables|Default|GetPlayerController)
      (:then
        (Default|MainSaveGametoPersistentMenu (Variables|/Game/CollaborativeViewer/Blueprints/PlayerController/BP_Collab_V_PlayerController.BP_Collab_V_PlayerController_C|GetSaveLoad_State_Controller _playercontroller))
        (bind _persistent_ui (Variables|/Game/CollaborativeViewer/Blueprints/PlayerController/BP_Collab_V_PlayerController.BP_Collab_V_PlayerController_C|GetPersistent_UI _playercontroller)
          (:then
            (bind _loadstatecombobox (Variables|/Game/CollaborativeViewer/UMG/GameMenu/Persistent_ToolBar.Persistent_ToolBar_C|GetLoadStateComboBox _persistent_ui)
              (:then
                (Default|AddOption _loadstatecombobox Value)
                (Default|SetSelectedOption _loadstatecombobox Value))
              (:else)))
          (:else)))
      (:else))))

(event EventOnGetComponents
  (bind _returnvalue (Game|GetPlayerController 0))
  ;[1 0.9636 0.2193] GetComponents
  (Utilities|IsValid _returnvalue
    (:Is%20Valid
      (bind _asbp_collab_v_player_controller (Utilities|Casting|CastToBP_Collab_V_PlayerController _returnvalue))
      (Variables|Default|SetPlayerController _asbp_collab_v_player_controller))))

(event EventSetupComplete
  ;[0.1454 1 0.1919] SetupComplete
  (Utilities|FlowControl|Sequence
    (:then_0
      (CallFunction|SetupBindings))))

(fn GetSaveGameDataJSon
  (params (Command :type String) (Action :type String))
  (bind _asbp_collab_v_player_controller (Utilities|Casting|CastToBP_Collab_V_PlayerController (Game|GetPlayerController 0))
    (:then
      (Default|AddtoMainSveGame (Variables|/Game/CollaborativeViewer/Blueprints/PlayerController/BP_Collab_V_PlayerController.BP_Collab_V_PlayerController_C|GetSaveLoad_State_Controller _asbp_collab_v_player_controller) (CallFunction|GetCurrentState)))
    (:CastFailed
      (CallFunction|PrintMissingComponent "Player Controller"))))

(fn MakeJsonProp
  (params (CommandType :type String) (Action :type String) (SaveGameData :type String))
  (bind _jsonobjectwrapper (Utilities|Struct|MakeJsonObjectWrapper))
  (|SetJsonField _jsonobjectwrapper "CurrentState" (CallFunction|GetCurrentState))
  (|SetJsonField _jsonobjectwrapper "Action" Action)
  (|SetJsonField _jsonobjectwrapper "Data" SaveGameData)
  (bind _outjsonstring (Class|JsonBlueprintFunctionLibrary|ToString _jsonobjectwrapper))
  (return _outjsonstring))

(fn GetCurrentState
  (bind _returnvalue (Class|CavrnusFunctionLibrary|GetStringPropertyValue (Variables|Default|GetSpace%20Connection) "State" "Current"))
  (return _returnvalue))

(fn GetCommand
  (params (InString :type String))
  (bind _outjsonobject (Class|JsonBlueprintFunctionLibrary|FromString InString))
  (bind _outvalue (|GetJsonField _outjsonobject "Command"))
  (return _outvalue))

(fn GetXrayJson)

(fn PrintMissingComponent
  (params (MissingComponent :type String))
  (Development|PrintString (Utilities|String|Append "AC_CavrnusStateManager: Cannot find " MissingComponent)))

(fn GetDimensionJson
  (bind _state (CallFunction|GetCurrentState))
  (bind _jsonobjectwrapper (Utilities|Struct|MakeJsonObjectWrapper))
  (Utilities|IsValid 0
    (:Is%20Valid
      (bind _output_get (LocalVariables|SetDimComponent 0))
      (Default|ToSaveGameROS _output_get _state)
      (bind _returnvalue (SaveGame|LoadGamefromSlot _state))
      (bind _asbp_data_save_game (Utilities|Casting|CastToBP_Data_SaveGame _returnvalue))
      (|SetJsonField _jsonobjectwrapper "DimLocations" (Variables|/Game/CollaborativeViewer/Blueprints/SaveGame/BP_Data_SaveGame.BP_Data_SaveGame_C|GetDimensionControlsLocation _asbp_data_save_game))
      (bind _outjsonstring (Class|JsonBlueprintFunctionLibrary|ToString _jsonobjectwrapper))
      (return _outjsonstring))
    (:Is%20Not%20Valid
      (CallFunction|PrintMissingComponent "Dimension Component"))))

(fn PostLocalSaveData
  (params (Command :type String) (Action :type String))
  (bind _outjsonstring (Data|GetSaveGameDataJSon Command Action))
  (Development|PrintString _outjsonstring))

(fn PostXrayData
  (params (Action :type String) (ToXray :type Boolean))
  (bind _jsonobjectwrapper (Utilities|Struct|MakeJsonObjectWrapper))
  (|SetJsonField _jsonobjectwrapper "CurrentState" (CallFunction|GetCurrentState))
  (|SetJsonField _jsonobjectwrapper "Action" Action))