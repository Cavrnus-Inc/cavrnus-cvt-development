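; Cavrnus command component that syncs X-ray effects on static mesh actors across a space through the pawn's BP_XrayComponent.
; Per-actor HasXray properties, keyed by CollabName_ tag, apply X-ray when true; the isolate binding also re-creates these bindings.
; Isolate (JSON actor list) and Reset are sent as transient updates cancelled immediately, acting as one-shot signals.
; Reset removes X-rays and clears any set HasXray flags.
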(event Custom|CreateXrayApplyBindings
  ;[1 1 1] Apply
  (for _array_element (Variables|Default|GetStaticMeshActors)
    (bind _returnvalue (Class|CavrnusFunctionLibrary|BindBooleanPropertyValue (Variables|Default|GetSpace%20Connection) (Utilities|String|Append "Xray/" (.ActorName (CallFunction|GetCollabTag _array_element "CollabName_"))) "HasXray" (delegate Custom|XrayUpdated)))
    (CallFunction|AddtoTrashCan _returnvalue)))

(event Custom|PostReset
  ;[1 1 1] PostReset
  (bind _returnvalue (Class|CavrnusFunctionLibrary|BeginTransientBoolPropertyUpdate (Variables|Default|GetSpace%20Connection) "Xray" "Reset" true))
  (Class|CavrnusLivePropertyUpdate|Cancel _returnvalue))

(event Custom|CustomEvent_0
  (params (Value :type String) (ContainerName :type String) (PropertyName :type String))
  ;[1 1 1] Isolate
  (bind _outjsonobject (Class|JsonBlueprintFunctionLibrary|FromString Value))
  (bind _outvalue (|GetJsonField _outjsonobject "Actors"))
  (bind _output_get (Variables|Default|SetIsolatedActors _outvalue))
  (for _array_element _output_get
    (Default|ApplyXrayROS (Variables|Default|GetXrayComponent) _array_element true)))

(event Custom|CreateResetBinding
  ;[1 1 1] Reset
  (bind _returnvalue (Class|CavrnusFunctionLibrary|BindBooleanPropertyValue (Variables|Default|GetSpace%20Connection) "Xray" "Reset" (delegate Custom|ResetXrays)))
  (CallFunction|AddtoTrashCan _returnvalue))

(event Custom|PostXrayUpdate
  (params (ActorName :type String) (Invisible :type Boolean))
  ;[1 1 1] PostXrayAction
  (Class|CavrnusFunctionLibrary|PostBoolPropertyUpdate (Variables|Default|GetSpace%20Connection) (Utilities|String|Append "Xray/" ActorName) "HasXray" Invisible))

(event Custom|XrayUpdated
  (params (Value :type Boolean) (ContainerName :type String) (PropertyName :type String))
  ;[1 1 1] Apply
  (if Value
    (Default|ApplyXrayROS (Variables|Default|GetXrayComponent) (Utilities|String|Replace ContainerName "Xray/") false)))

(event Custom|PostIsolateXray
  (params (Actors :type Array%20of%20Strings))
  (bind _jsonobjectwrapper (Utilities|Struct|MakeJsonObjectWrapper))
  ;[1 1 1] PostReset
  (|SetJsonField _jsonobjectwrapper "Actors" Actors)
  (bind _outjsonstring (Class|JsonBlueprintFunctionLibrary|ToString _jsonobjectwrapper))
  (bind _returnvalue (Class|CavrnusFunctionLibrary|BeginTransientStringPropertyUpdate (Variables|Default|GetSpace%20Connection) "Xray" "Isolate" _outjsonstring))
  (Class|CavrnusLivePropertyUpdate|Cancel _returnvalue))

(event Custom|CreateIsolateBinding
  ;[1 1 1] Isolate
  (bind _returnvalue (Class|CavrnusFunctionLibrary|BindStringPropertyValue (Variables|Default|GetSpace%20Connection) "Xray" "Isolate" (delegate Custom|CustomEvent_0)))
  (CallFunction|AddtoTrashCan _returnvalue)
  (CallFunction|CreateXrayApplyBindings))

(event Custom|ResetXrays
  (params (Value :type Boolean) (ContainerName :type String) (PropertyName :type String))
  (bind _space_connection (Variables|Default|GetSpace%20Connection))
  ;[1 1 1] Reset
  (if Value
    (Default|RemoveXrayROS (Variables|Default|GetXrayComponent) false)
    (for _array_element (Variables|Default|GetStaticMeshActors)
      (bind _returnvalue (Class|CavrnusFunctionLibrary|GetBoolPropertyValue _space_connection (Utilities|String|Append "Xray/" (.ActorName (CallFunction|GetCollabTag _array_element "CollabName_"))) "HasXray"))
      (if _returnvalue
        (Class|CavrnusFunctionLibrary|PostBoolPropertyUpdate _space_connection (Utilities|String|Append "Xray/" (.ActorName (CallFunction|GetCollabTag _array_element "CollabName_"))) "HasXray" false)))))

(event Custom|SetupXrayBindings
  ;[1 1 1] Setup Bindings
  (Utilities|FlowControl|Sequence
    (:then_0
      (CallFunction|CreateXrayApplyBindings))
    (:then_1
      (CallFunction|CreateResetBinding))
    (:then_2
      (CallFunction|CreateIsolateBinding))))

(event EventOnGetComponents
  (bind _pawn (Variables|Default|GetPawn))
  (bind _returnvalue (Actor|GetComponentbyClass _pawn "/Game/CollaborativeViewer/Blueprints/Commands/Xray/BP_XrayComponent.BP_XrayComponent_C"))
  ;[0.1454 1 0.1919] OnGetComponents
  (Utilities|IsValid _returnvalue
    (:Is%20Valid
      (bind _output_get (Variables|Default|SetXrayComponent _returnvalue))
      (Variables|Default|SetXrayManager (Variables|/Game/CollaborativeViewer/Blueprints/Commands/Xray/BP_XrayComponent.BP_XrayComponent_C|GetXrayManager _output_get))
      (bind _outactors (Actor|GetAllActorsOfClass "/Script/Engine.StaticMeshActor"))
      (Variables|Default|SetStaticMeshActors _outactors))
    (:Is%20Not%20Valid
      (Development|PrintString "AC_Cavrnus_SyncXray: XrayComponent not found on Pawn!"))))

(event EventOnSetupComplete
  ;[1 0.9636 0.2193] SetupComplete
  (CallFunction|SetupXrayBindings))