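; Actor component that syncs X-ray tool actions across a Cavrnus space for the locally controlled BP_BasePawn.
; On space connection, it binds to the pawn's BP_XrayComponent and posts each action as single-field JSON to a shared string property.
; Property updates are parsed back into Apply, Isolate or Reset calls on that component.
; Reset posts an empty Apply value, then begins and immediately cancels a transient Reset update.
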(event Custom|SpaceConnected
  (params (SpaceConnection :type Cavrnus%20Space%20Connection%20Structure))
  (bind _returnvalue (Components|GetOwner))
  (bind _returnvalue_2 (Actor|GetComponentbyClass _returnvalue "/Game/CollaborativeViewer/Blueprints/Commands/Xray/BP_XrayComponent.BP_XrayComponent_C"))
  (bind _asbp_base_pawn (Utilities|Casting|CastToBP_BasePawn (Components|GetOwner)))
  (if (Pawn|IsLocallyControlled _asbp_base_pawn)
    (Variables|Default|SetSpaceConnection SpaceConnection)
    (Utilities|FlowControl|Delay 0.2)
    (Utilities|IsValid _returnvalue
      (:Is%20Valid
        (Utilities|IsValid _returnvalue_2
          (:Is%20Valid
            (bind _output_get (Variables|Default|SetXrayComponent _returnvalue_2))
            (Variables|Default|SetXrayManager (Variables|/Game/CollaborativeViewer/Blueprints/Commands/Xray/BP_XrayComponent.BP_XrayComponent_C|GetXrayManager _output_get))
            (Variables|Default|GetXrayManager
              (:then
                (CallFunction|SetupXrayBindings))
              (:else))))))))

(event Custom|Updated
  (params (Value :type String) (ContainerName :type String) (PropertyName :type String))
  (bind _xraycomponent (Variables|Default|GetXrayComponent))
  ;[1 1 1] Setup Bindings
  (if (not (Utilities|Array|IsEmpty Value))
    (bind _actiontype (CallFunction|GetActionType Value))
    (bind _actors (CallFunction|GetModifiedActorsArray Value))
    (switch string _actiontype
      (:Default
        (Development|PrintString (Utilities|String|Append "XRay Action Invalid:" Value)))
      (:Apply
        (for _array_element _actors
          (Default|ApplyXrayROS (Variables|Default|GetXrayComponent) _array_element)))
      (:Isolate
        (Default|IsolateXrayROS (Variables|Default|GetXrayComponent) _actors))
      (:Reset
        (Default|RemoveXrayROS _xraycomponent)
        (Default|UpdateCropBoxROS _xraycomponent)))))

(event Custom|ActionPerformed
  (params (ActionType :type String) (ModifiedActors :type Array%20of%20Strings))
  ;[1 1 1] Setup Bindings
  (CallFunction|PostModifiedActors ActionType ModifiedActors))

(event Custom|SetupXrayBindings
  ;[1 1 1] Setup Bindings
  (EventDispatchers|BindEventtoCavrnusXrayActionPerformed (Variables|Default|GetXrayComponent) (delegate Custom|ActionPerformed))
  (Class|CavrnusFunctionLibrary|BindStringPropertyValue (Variables|Default|GetSpaceConnection) "XrayTool" "Action" (delegate Custom|Updated)))

(event EventBeginPlay
  (Class|CavrnusFunctionLibrary|AwaitAnySpaceConnection (delegate Custom|SpaceConnected)))

(fn PostModifiedActors
  (params (ActionType :type String) (ModifiedTransforms :type Array%20of%20Strings))
  (bind _jsonobjectwrapper (Utilities|Struct|MakeJsonObjectWrapper))
  (|SetJsonField _jsonobjectwrapper ActionType ModifiedTransforms)
  (bind _outjsonstring (Class|JsonBlueprintFunctionLibrary|ToString _jsonobjectwrapper))
  (switch string ActionType
    (:Apply
      (Class|CavrnusFunctionLibrary|PostStringPropertyUpdate (Variables|Default|GetSpaceConnection) "XrayTool" "Action" _outjsonstring :!label _label))
    (:Isolate
      (goto _label))
    (:Reset
      (Class|CavrnusFunctionLibrary|PostStringPropertyUpdate (Variables|Default|GetSpaceConnection) "XrayTool" "Action" "Apply\":[]")
      (bind _returnvalue (Class|CavrnusFunctionLibrary|BeginTransientStringPropertyUpdate (Variables|Default|GetSpaceConnection) "XrayTool" "Action" _outjsonstring))
      (Class|CavrnusLivePropertyUpdate|Cancel _returnvalue))))

(fn GetModifiedActorsArray
  (params (InJsonString :type String))
  (bind (_outjsonobject _returnvalue) (Class|JsonBlueprintFunctionLibrary|FromString InJsonString))
  (if _returnvalue
    (bind (_fieldnames _returnvalue_2) (Class|JsonBlueprintFunctionLibrary|GetFieldNames _outjsonobject))
    (if _returnvalue_2
      (bind (_outvalue _returnvalue_3) (|GetJsonField _outjsonobject (Utilities|Array|Get(acopy) _fieldnames)))
      (if _returnvalue_3
        (return _outvalue)))))

(fn GetActionType
  (params (InJsonString :type String))
  (bind (_outjsonobject _returnvalue) (Class|JsonBlueprintFunctionLibrary|FromString InJsonString))
  (if _returnvalue
    (bind (_fieldnames _returnvalue_2) (Class|JsonBlueprintFunctionLibrary|GetFieldNames _outjsonobject))
    (if _returnvalue_2
      (return (Utilities|Array|Get(acopy) _fieldnames)))))