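; Actor component that turns a Cavrnus-spawned object into a local bookmark in the player's bookmark UI and save data.
; On space connection, it finds the pawn's BP_BookmarkComponent and binds the container's "Bookmark" string property, parsing its JSON into name and transform.
; Updates create a bookmark through the bookmark manager.
; Deletion is mirrored: destroying the level bookmark destroys the Cavrnus object, while destroying the owner removes the bookmark's UI, actor and save entry.
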(event Custom|SetupBindings
  ;[1 1 1] SetupBindings
  (Class|CavrnusFunctionLibrary|BindStringPropertyValue (Variables|Default|GetSpace%20Connection) (Variables|Default|GetContainer%20Name) "Bookmark" (delegate Custom|BookmarkUpdate)))

(event Custom|AddToUI
  ;[1 1 1] AddToUI
  (bind _bookmarkcomponent (Variables|Default|GetBookmarkComponent)
    (:then
      (bind _managerbookmark (Variables|/Game/CollaborativeViewer/Blueprints/Commands/Bookmark/BP_BookmarkComponent.BP_BookmarkComponent_C|GetManagerBookmark _bookmarkcomponent)
        (:then
          (bind _bookmarksavegame (Variables|/Game/CollaborativeViewer/Blueprints/Commands/Bookmark/UMG/BookMarkManager.BookMarkManager_C|GetBookMarkSaveGame _managerbookmark)
            (:then
              (bind _bookmark (Default|CreateBookmark _managerbookmark (Utilities|Text|ToText(String) (Variables|Default|GetBookmarkName)) _bookmarksavegame (Variables|Default|GetBookmarkTransform)))
              (bind _output_get (Variables|Default|SetSpawnedBookMark _bookmark))
              (Rendering|Components|TextRender|SetText (Variables|/Game/CollaborativeViewer/Blueprints/Commands/Bookmark/UMG/BookMarkManager.BookMarkManager_C|GetBookmarkTextMulti (Variables|/Game/CollaborativeViewer/Blueprints/Commands/Bookmark/BP_BookmarkComponent.BP_BookmarkComponent_C|GetManagerBookmark (Variables|Default|GetBookmarkComponent))) "")
              (Game|BindEventtoOnDestroyed (Variables|/Game/CollaborativeViewer/Blueprints/Commands/Bookmark/UMG/AddedBookmarkWidget.AddedBookmarkWidget_C|GetLevelBookMark _output_get) (delegate Custom|Destroyed))
              (Default|CreateBookMark (Variables|Default|GetBookmarkComponent) "" _output_get)
              (Game|BindEventtoOnDestroyed (delegate Custom|RemotelyDestroyed)))
            (:else)))
        (:else)))
    (:else)))

(event Custom|BookmarkUpdate
  (params (Value :type String) (ContainerName :type String) (PropertyName :type String))
  ;[1 1 1] SetupBindings
  (bind (_outjsonobject _returnvalue) (Class|JsonBlueprintFunctionLibrary|FromString Value))
  (if _returnvalue
    (bind (_outvalue _returnvalue_2) (|GetJsonField _outjsonobject "Name"))
    (if _returnvalue_2
      (Variables|Default|SetBookmarkName _outvalue)
      (bind (_outvalue_2 _returnvalue_3) (|GetJsonField _outjsonobject "Transform"))
      (if _returnvalue_3
        (Variables|Default|SetBookmarkTransform _outvalue_2)
        (CallFunction|AddtoUI)))))

(event Custom|RemotelyDestroyed
  (params (DestroyedActor :type Actor%20Object%20Reference))
  ;[1 1 1] AddToUI
  (bind _bookmarksavegame (Utilities|RemoveBookmark (Variables|Default|GetSpawnedBookMark)))
  (SaveGame|SaveGametoSlot _bookmarksavegame "Bookmarks")
  (bind _spawnedbookmark (Variables|Default|GetSpawnedBookMark)
    (:then
      (bind _levelbookmark (Variables|/Game/CollaborativeViewer/Blueprints/Commands/Bookmark/UMG/AddedBookmarkWidget.AddedBookmarkWidget_C|GetLevelBookMark _spawnedbookmark)
        (:then
          (Utilities|FlowControl|Sequence
            (:then_0
              (bind _optionbutton (Variables|/Game/CollaborativeViewer/Blueprints/Commands/Bookmark/BPs/BP_Bookmark.BP_Bookmark_C|GetOPtionButton _levelbookmark)
                (:then
                  (Widget|RemovefromParent _optionbutton))
                (:else)))
            (:then_1
              (bind _cavrnus_listitem (Variables|/Game/CollaborativeViewer/Blueprints/Commands/Bookmark/BPs/BP_Bookmark.BP_Bookmark_C|GetCavrnus_ListItem _levelbookmark)
                (:then
                  (Widget|RemovefromParent _cavrnus_listitem))
                (:else)))
            (:then_2
              (Actor|DestroyActor _levelbookmark))))
        (:else)))
    (:else)))

(event Custom|Destroyed
  (params (DestroyedActor :type Actor%20Object%20Reference))
  ;[1 1 1] AddToUI
  (Class|CavrnusFunctionLibrary|DestroyObject (Variables|/Script/CavrnusConnector.CavrnusSpawnedObjectFlag|GetSpawnedObject (Variables|Default|GetSpawnedObjFlag))))

(event Custom|SpaceConnected
  (params (SpaceConnection :type Cavrnus%20Space%20Connection%20Structure))
  (bind _returnvalue (Actor|GetComponentbyClass "/Script/CavrnusConnector.CavrnusPropertiesContainer"))
  (Variables|Default|SetSpace%20Connection SpaceConnection)
  (Utilities|FlowControl|Delay 0.0)
  (Utilities|IsValid _returnvalue
    (:Is%20Valid
      (Variables|Default|SetContainer%20Name (Variables|/Script/CavrnusConnector.CavrnusPropertiesContainer|GetContainerName _returnvalue))
      (Variables|Default|SetSpawnedObjFlag (Actor|GetComponentbyClass "/Script/CavrnusConnector.CavrnusSpawnedObjectFlag"))
      (Variables|Default|GetSpawnedObjFlag
        (:then
          (bind _asbp_base_pawn (Utilities|Casting|CastToBP_BasePawn (Game|Player|GetPlayerPawn 0))
            (:then
              (Variables|Default|SetBookmarkComponent (Actor|GetComponentbyClass _asbp_base_pawn "/Game/CollaborativeViewer/Blueprints/Commands/Bookmark/BP_BookmarkComponent.BP_BookmarkComponent_C"))
              (Variables|Default|GetBookmarkComponent
                (:then
                  (Utilities|FlowControl|Sequence
                    (:then_0
                      (CallFunction|SetupBindings))))
                (:else
                  (Development|PrintString "Hello[AC_Cavrnus_BookmarkLoader] Unable to find BP_BookmarkComponent!"))))
            (:CastFailed
              (Development|PrintString "[AC_Cavrnus_BookmarkLoader] Unable to cast to BasePawn!"))))
        (:else
          (Development|PrintString "[AC_Cavrnus_BookmarkLoader] Unable to cast to BasePawn!"))))))

(event EventBeginPlay
  (Class|CavrnusFunctionLibrary|AwaitAnySpaceConnection (delegate Custom|SpaceConnected)))

(fn ConstructionScript)