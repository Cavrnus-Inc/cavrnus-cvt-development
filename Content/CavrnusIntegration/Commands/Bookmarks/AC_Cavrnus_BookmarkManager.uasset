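; Pawn component that publishes newly created bookmarks to a Cavrnus space, active only on a locally controlled BP_BasePawn.
; Once the space connects, it waits briefly, finds the owner's BP_BookmarkComponent and binds to its manager's bookmark-created event.
; Each creation spawns a BP_Cavrnus_BookmarkLoader object and posts name and transform as a JSON string to its Bookmark property.
; The transform comes from the current player camera; the event's Location argument is unused.
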(event Custom|SpaceConnected
  (params (SpaceConnection :type Cavrnus%20Space%20Connection%20Structure))
  (bind _returnvalue (Components|GetOwner))
  (bind _returnvalue_2 (Actor|GetComponentbyClass _returnvalue "/Game/CollaborativeViewer/Blueprints/Commands/Bookmark/BP_BookmarkComponent.BP_BookmarkComponent_C"))
  (bind _asbp_base_pawn (Utilities|Casting|CastToBP_BasePawn (Components|GetOwner)))
  (if (Pawn|IsLocallyControlled _asbp_base_pawn)
    (Variables|Default|SetPawn _asbp_base_pawn)
    (Variables|Default|SetSpaceConnection SpaceConnection)
    (Utilities|FlowControl|Delay 0.2)
    (Utilities|IsValid _returnvalue
      (:Is%20Valid
        (Utilities|IsValid _returnvalue_2
          (:Is%20Valid
            (Variables|Default|SetBookmarkComponent _returnvalue_2)
            (CallFunction|SetupComponent)))))))

(event Custom|SetupComponent
  (EventDispatchers|BindEventtoCavrnusBookmarkCreated (Variables|/Game/CollaborativeViewer/Blueprints/Commands/Bookmark/BP_BookmarkComponent.BP_BookmarkComponent_C|GetManagerBookmark (Variables|Default|GetBookmarkComponent)) (delegate Custom|Created)))

(event Custom|Created
  (params (Text :type Text) (Location :type Transform))
  (CallFunction|PostBookmark Text Location))

(event EventBeginPlay
  (Class|CavrnusFunctionLibrary|AwaitAnySpaceConnection (delegate Custom|SpaceConnected)))

(fn PostBookmark
  (params (Text :type Text) (Location :type Transform))
  (bind _returnvalue (Game|GetPlayerController 0))
  (bind _jsonobjectwrapper (Utilities|Struct|MakeJsonObjectWrapper))
  (bind _playercameramanager (Variables|/Script/Engine.PlayerController|GetPlayerCameraManager _returnvalue))
  (bind _returnvalue_2 (Class|CavrnusFunctionLibrary|SpawnObject (Variables|Default|GetSpaceConnection) "BP_Cavrnus_BookmarkLoader"))
  (|SetJsonField _jsonobjectwrapper "Name" (Utilities|Text|ToText(String) (Utilities|String|ToString(Text) Text)))
  (|SetJsonField _jsonobjectwrapper "Transform" (Math|Transform|MakeTransform (Camera|GetCameraLocation _playercameramanager) (Camera|GetCameraRotation _playercameramanager)))
  (bind _outjsonstring (Class|JsonBlueprintFunctionLibrary|ToString _jsonobjectwrapper))
  (Class|CavrnusFunctionLibrary|PostStringPropertyUpdate (Variables|Default|GetSpaceConnection) (.propertiescontainername _returnvalue_2) "Bookmark" _outjsonstring))