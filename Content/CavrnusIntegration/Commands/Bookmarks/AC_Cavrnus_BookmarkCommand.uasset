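; Cavrnus command component that shares newly created bookmarks with the connected space.
; It finds the pawn's BP_BookmarkComponent and binds to its bookmark manager's created event.
; Each bookmark spawns a BP_Cavrnus_BookmarkLoader object in the space, then posts name and camera transform as a JSON string to that object's "Bookmark" property.
; The transform comes from the player camera's location and rotation; the event's Location argument is unused.
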(event Custom|SetupBindings
  ;[1 1 1] SetupBindings
  (EventDispatchers|BindEventtoCavrnusBookmarkCreated (Variables|/Game/CollaborativeViewer/Blueprints/Commands/Bookmark/BP_BookmarkComponent.BP_BookmarkComponent_C|GetManagerBookmark (Variables|Default|GetBookmarkComponent)) (delegate Custom|Created)))

(event Custom|Created
  (params (Text :type Text) (Location :type Transform))
  ;[1 1 1] SetupBindings
  (CallFunction|PostBookmark Text Location))

(event EventOnGetComponents
  (bind _pawn (Variables|Default|GetPawn))
  (bind _returnvalue (Actor|GetComponentbyClass _pawn "/Game/CollaborativeViewer/Blueprints/Commands/Bookmark/BP_BookmarkComponent.BP_BookmarkComponent_C"))
  ;[1 0.9636 0.2193] GetComponents
  (Utilities|IsValid _returnvalue
    (:Is%20Valid
      (Variables|Default|SetBookmarkComponent _returnvalue))))

(event EventOnSetupComplete
  ;[0.1454 1 0.1919] OnSetupComplete
  (CallFunction|SetupBindings))

(fn PostBookmark
  (params (Text :type Text) (Location :type Transform))
  (bind _jsonobjectwrapper (Utilities|Struct|MakeJsonObjectWrapper))
  (bind _playercontroller (Variables|Default|GetPlayerController))
  (bind _playercameramanager (Variables|/Script/Engine.PlayerController|GetPlayerCameraManager _playercontroller))
  (bind _returnvalue (Class|CavrnusFunctionLibrary|SpawnObject (Variables|Default|GetSpace%20Connection) "BP_Cavrnus_BookmarkLoader"))
  (|SetJsonField _jsonobjectwrapper "Name" (Utilities|Text|ToText(String) (Utilities|String|ToString(Text) Text)))
  (|SetJsonField _jsonobjectwrapper "Transform" (Math|Transform|MakeTransform (Camera|GetCameraLocation _playercameramanager) (Camera|GetCameraRotation _playercameramanager)))
  (bind _outjsonstring (Class|JsonBlueprintFunctionLibrary|ToString _jsonobjectwrapper))
  (Class|CavrnusFunctionLibrary|PostStringPropertyUpdate (Variables|Default|GetSpace%20Connection) (.propertiescontainername _returnvalue) "Bookmark" _outjsonstring))