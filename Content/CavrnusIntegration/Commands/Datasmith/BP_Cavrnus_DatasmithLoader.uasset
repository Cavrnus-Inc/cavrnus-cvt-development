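; Cavrnus-spawned actor that loads a shared Datasmith file into the space.
; It binds DatasmithFile and Transform properties, then downloads the zip by content ID behind a progress visualizer, unzips it and finds the .udatasmith.
; It simulates a selection in the pawn's Datasmith toolbar to add an anchor, unless already loaded, and attaches transform-sync components.
; Destroy handlers propagate removal between anchor and spawned object and delete the local folder.
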(event Custom|OnSpaceConnected
  (params (SpaceConnection :type Cavrnus%20Space%20Connection%20Structure))
  (bind _returnvalue (Actor|GetComponentbyClass "/Script/CavrnusConnector.CavrnusPropertiesContainer"))
  ;[0.03817 1 0.05703] BeginPlay
  (Variables|Default|SetSpaceConnection SpaceConnection)
  (Utilities|FlowControl|Delay 0.0)
  (Utilities|IsValid _returnvalue
    (:Is%20Valid
      (Variables|Default|SetContainerName (Variables|/Script/CavrnusConnector.CavrnusPropertiesContainer|GetContainerName _returnvalue))
      (bind _asbp_base_pawn (Utilities|Casting|CastToBP_BasePawn (Game|Player|GetPlayerPawn 0))
        (:then
          (Variables|Default|SetDatasmithComponent (Actor|GetComponentbyClass _asbp_base_pawn "/Game/CollaborativeViewer/Blueprints/Commands/DataSmith/BP_DataSmith_Component.BP_DataSmith_Component_C"))
          (Utilities|FlowControl|Sequence
            (:then_0
              (CallFunction|SetupBindings))))
        (:CastFailed
          (Development|PrintString "Unable to find Datasmith Component!"))))))

(event Custom|DownloadComplete
  (params (fileDest :type String))
  ;[1 1 1] FetchFileById
  (Default|FinalizeLoading (Variables|Default|GetLoaderWidget))
  (bind (_archivefilelocation _diskfilelocation) (|UnzipZipArchive fileDest (Variables|Default|GetSaveLocation) "" true)
    (:OnArchiveUnzipped
      (bind _output (Utilities|FileProcessing _diskfilelocation _archivefilelocation))
      (CallFunction|LoadfromAnchor _output))))

(event Custom|PropertySetup
  (params (StringValue :type String))
  ;[1 1 1] ProcessJson and SetVariables
  (bind (_outjsonobject _returnvalue) (Class|JsonBlueprintFunctionLibrary|FromString StringValue))
  (if _returnvalue
    (bind (_outvalue _returnvalue_2) (|GetJsonField _outjsonobject "UploadedFile"))
    (if _returnvalue_2
      (Variables|Default|SetContentId _outvalue)
      (Variables|Default|SetSaveLocation (Utilities|String|Append (Class|FilePaths|GetSavedFolder "CavrnusDownloads") "/" _outvalue))
      (bind _returnvalue_3 (Utilities|SpawnLoaderWidget (Variables|Default|GetSpaceConnection) (Variables|Default|GetContainerName)))
      (Variables|Default|SetLoaderWidget _returnvalue_3)
      (CallFunction|FetchFilebyId))))

(event Custom|TransformUpdated
  (params (Value :type Transform) (ContainerName :type String) (PropertyName :type String))
  ;[1 1 1] SetupBindings
  (bind _endpoint_ui (Variables|Default|GetEndpoint%20UI)
    (:then
      (Default|SetTextLocation _endpoint_ui (.Location (Math|Transform|BreakTransform Value))))
    (:else)))

(event Custom|OnDestroyedEvent
  (params (DestroyedActor :type Actor%20Object%20Reference))
  (bind _returnvalue (Actor|GetComponentbyClass "/Script/CavrnusConnector.CavrnusSpawnedObjectFlag"))
  ;[1 1 1] HandleSpawnedActor
  ;;[1 1 1] Handle OnDestroy
  (Utilities|IsValid _returnvalue
    (:Is%20Valid
      (Class|CavrnusFunctionLibrary|DestroyObject (Variables|/Script/CavrnusConnector.CavrnusSpawnedObjectFlag|GetSpawnedObject _returnvalue))
      (Class|FilePaths|DeleteLocalFolder (Variables|Default|GetSaveLocation)))))

(event Custom|SetupBindings
  ;[1 1 1] SetupBindings
  (Class|CavrnusFunctionLibrary|BindStringPropertyValue (Variables|Default|GetSpaceConnection) (Variables|Default|GetContainerName) "DatasmithFile" (delegate Custom|PropertyReceived))
  (Class|CavrnusFunctionLibrary|BindTransformPropertyValue (Variables|Default|GetSpaceConnection) (Variables|Default|GetContainerName) "Transform" (delegate Custom|TransformUpdated)))

(event Custom|PropertyReceived
  (params (Value :type String) (ContainerName :type String) (PropertyName :type String))
  ;[1 1 1] SetupBindings
  (CallFunction|PropertySetup Value))

(event Custom|LoadFromAnchor
  (params (Path :type String))
  (bind _datasmithcomponent (Variables|Default|GetDatasmithComponent))
  (bind _datasmith_toolbar (Variables|/Game/CollaborativeViewer/Blueprints/Commands/DataSmith/BP_DataSmith_Component.BP_DataSmith_Component_C|GetDatasmith_Toolbar _datasmithcomponent))
  ;[1 1 1] Load File via CVT - User their anchor logic
  (bind (_wasloaded _anchor) (CallFunction|IsAlreadyLoaded Path))
  (if _wasloaded
    (CallFunction|HandleSpawnedActor _anchor)
    (else
      ;;[1 1 1] Basically simulates clicking on the UI entry
      (Variables|/Game/CollaborativeViewer/Blueprints/Commands/DataSmith/UMG/DRToolbarUI.DRToolbarUI_C|SetCurrentFilePath _datasmith_toolbar Path)
      (bind _returnvalue (Class|CavrnusFunctionLibrary|GetTransformPropertyValue (Variables|Default|GetSpaceConnection) (Variables|Default|GetContainerName) "Transform"))
      (bind (_spawnedactor _endpointui) (Default|AddAnchor _datasmith_toolbar _returnvalue))
      (Variables|Default|SetEndpoint%20UI _endpointui)
      (Variables|Default|SetSpawned%20Actor _spawnedactor)
      (Default|SetAnchor _endpointui _spawnedactor)
      (Default|LoadingDataSmithStarted _endpointui)
      (CallFunction|HandleSpawnedActor _spawnedactor)))
  ;;[1 1 1] Important! Clear out the selection
  (Variables|/Game/CollaborativeViewer/Blueprints/Commands/DataSmith/UMG/DRToolbarUI.DRToolbarUI_C|SetCurrentFilePath (Variables|/Game/CollaborativeViewer/Blueprints/Commands/DataSmith/BP_DataSmith_Component.BP_DataSmith_Component_C|GetDatasmith_Toolbar (Variables|Default|GetDatasmithComponent)) ""))

(event Custom|DestroyedRemotely
  (params (DestroyedActor :type Actor%20Object%20Reference))
  ;[1 1 1] HandleSpawnedActor
  ;;[1 1 1] Handle OnDestroy
  (Variables|Default|GetSpawned%20Actor
    (:then
      (Actor|DestroyActor)
      (Class|FilePaths|DeleteLocalFolder (Variables|Default|GetSaveLocation)))
    (:else)))

(event Custom|FetchFileById
  ;[1 1 1] FetchFileById
  (Class|CavrnusFunctionLibrary|FetchFilebyIdtoDisk (Variables|Default|GetContentId) (Variables|Default|GetSaveLocation) (delegate Custom|OnProgress) (delegate Custom|DownloadComplete)))

(event Custom|OnProgress
  (params (Progress :type Float%20%28single-precision%29) (Step :type String))
  ;[1 1 1] FetchFileById
  (Utilities|UpdateLoaderWidget Progress))

(event Custom|HandleSpawnedActor
  (params (TargetActor :type Datasmith%20Runtime%20Actor%20Object%20Reference))
  ;[1 1 1] HandleSpawnedActor
  (Utilities|IsValid TargetActor
    (:Is%20Valid
      (Utilities|FlowControl|Sequence
        (:then_0
          (Utilities|AddSyncTransform TargetActor))
        (:then_1
          ;;[1 1 1] Handle OnDestroy
          (Game|AssignOnDestroyed TargetActor (delegate Custom|OnDestroyedEvent))
          (Game|BindEventtoOnDestroyed (delegate Custom|DestroyedRemotely)))))))

(event EventBeginPlay
  ;[0.03817 1 0.05703] BeginPlay
  (Class|CavrnusFunctionLibrary|AwaitAnySpaceConnection (delegate Custom|OnSpaceConnected)))

(fn ConstructionScript)