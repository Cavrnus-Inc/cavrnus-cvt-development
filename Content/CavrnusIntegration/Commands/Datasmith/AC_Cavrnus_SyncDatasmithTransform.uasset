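; Actor component in the Cavrnus integration that exposes a Datasmith actor's mesh transform for property syncing.
; From BeginPlay it retries on a short delay until the first child of the owner's root component is a static mesh, then caches it.
; SetTransform applies the incoming property value as that mesh's world transform, and GetTransform returns it, both only when the mesh is valid.
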(event EventSetTransform
  (params (PropertyValue :type Transform))
  (bind _mesh (Variables|Default|GetMesh)
    (:then
      (Transformation|SetWorldTransform _mesh PropertyValue false false))
    (:else)))

(event EventBeginPlay
  (bind _returnvalue (Components|GetOwner))
  (bind _rootcomponent (Variables|/Script/Engine.Actor|GetRootComponent _returnvalue))
  (bind _children (Components|GetChildrenComponents _rootcomponent true))
  (Utilities|FlowControl|Delay 0.0)
  (if (Utilities|Array|IsNotEmpty _children) :!label _label
    (bind _asstatic_mesh_component (Utilities|Casting|CastToStaticMeshComponent (Utilities|Array|Get(acopy) _children))
      (:then
        (Variables|Default|SetMesh _asstatic_mesh_component))
      (:CastFailed
        (Utilities|FlowControl|Delay 0.2 :!label _label_2)
        (goto _label)))
    (else
      (goto _label_2))))

(fn GetTransform
  (bind _mesh (Variables|Default|GetMesh)
    (:then
      (return (Transformation|GetWorldTransform _mesh)))
    (:else)))