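; Remote-player pawn for Orbit navigation mode in the Cavrnus integration, extending a parent pawn.
; BeginPlay sets the Orbit navigation icon and fills the player mesh array before running parent logic, while Tick re-hides the main Mesh and its children every frame.
; The construction script attaches VisualOpacityOverlap to the Camera, and a GetHit helper returns a complex cursor trace against static and dynamic world objects.
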(event EventBeginPlay
  ;[0.0146 1 0] Begin play
  (Variables|Default|SetNavigationIconTexture "/Game/CollaborativeViewer/UMG/Textures/Orbit.Orbit")
  (Variables|Default|SetPlayerMeshesArray (Utilities|Array|MakeArray (Variables|Character|GetMesh) (Variables|Default|GetStaticMesh)))
  (|CallParentFunction))

(event EventTick
  (params (DeltaSeconds :type Float%20%28single-precision%29))
  ;[1 0 0] Tick
  (|CallParentFunction DeltaSeconds)
  (Rendering|SetVisibility (Variables|Character|GetMesh) false true))

(fn ConstructionScript
  (Transformation|AttachComponentToComponent (Variables|Default|GetVisualOpacityOverlap) (Variables|Default|GetCamera) "None" "KeepRelative" "KeepRelative" "KeepRelative" true))

(fn GetHit
  (return (.HitResult (Class|PlayerController|GetHitResultUnderCursorforObjects (Game|GetPlayerController 0) (Utilities|Array|MakeArray "ObjectTypeQuery1" "ObjectTypeQuery2") true))))