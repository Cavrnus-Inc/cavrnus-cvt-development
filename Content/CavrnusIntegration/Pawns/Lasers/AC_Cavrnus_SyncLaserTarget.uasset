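; Actor component that syncs a BP_BasePawn's laser pointer target location across a Cavrnus space.
; Once connected, it reads the pawn's properties container and branches on local control.
; Local pawns stream target spawns into a transient "LaserTarget" vector property; the first spawn only creates the updater.
; Remote pawns bind that property and spawn a BP_LaserPointerTarget in the player's color, skipping values with any zero axis.
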(event Custom|SpaceConnected
  (params (SpaceConnection :type Cavrnus%20Space%20Connection%20Structure))
  (bind _returnvalue (Components|GetOwner))
  ;[0.006856 1 0] Setup - Get specified Laser
  (Variables|Default|SetSpace%20Connection SpaceConnection)
  ;;[0.006856 1 0] Wait to grab properties container
  (Utilities|FlowControl|Delay 0.0)
  (Utilities|IsValid _returnvalue
    (:Is%20Valid
      (bind _asbp_base_pawn (Utilities|Casting|CastToBP_BasePawn _returnvalue)
        (:then
          (bind _output_get (Variables|Default|SetOwner _asbp_base_pawn))
          (Variables|Default|SetContainerName (Variables|/Script/CavrnusConnector.CavrnusPropertiesContainer|GetContainerName (Actor|GetComponentbyClass _output_get "/Script/CavrnusConnector.CavrnusPropertiesContainer")))
          (if (Pawn|IsLocallyControlled _output_get)
            (CallFunction|BindSendProperty)
            (else
              (CallFunction|BindRecieveProperty))))
        (:CastFailed
          (Development|PrintString "[AC_Cavrnus_SyncLaserTarget] Failed casting to BP_BasePawn!"))))))

(event Custom|TargetSpawned
  (params (SpawnLocation :type Transform))
  ;[1 1 1] Bind SendProperty for local users
  (bind _updater (Variables|Default|GetUpdater)
    (:then
      (Class|CavrnusLiveVectorPropertyUpdate|UpdatewithNewData _updater (Math|Conversions|ToVector(Vector4) (Math|Vector4|MakeVector4 (.x (.location SpawnLocation)) (.y (.location SpawnLocation)) (.z (.location SpawnLocation)) 0.0))))
    (:else
      (bind _returnvalue (Class|CavrnusFunctionLibrary|BeginTransientVectorPropertyUpdate (Variables|Default|GetSpace%20Connection) (Variables|Default|GetContainerName) "LaserTarget"))
      (Variables|Default|SetUpdater _returnvalue))))

(event Custom|CustomEvent_0
  (params (Value :type Vector%204%20Structure) (ContainerName :type String) (PropertyName :type String))
  ;[1 1 1] Bind ReceiveProperty from remote users
  (if (!= (.x Value) 0.0)
    (if (!= (.y Value) 0.0)
      (if (!= (.z Value) 0.0)
        (Game|SpawnActorfromClass "/Game/CollaborativeViewer/Blueprints/LaserPointerTarget/BP_LaserPointerTarget.BP_LaserPointerTarget_C" (Math|Transform|MakeTransform (Math|Vector|MakeVector (.x Value) (.y Value) (.z Value)) "0, 0, 0" "1.000000,1.000000,1.000000") "Undefined" "OverrideRootScale" 0 2.0 8.0 (Variables|/Game/CollaborativeViewer/Blueprints/Pawn/BP_BasePawn.BP_BasePawn_C|GetPlayerColor (Variables|Default|GetOwner)) 0)))))

(event Custom|BindSendProperty
  ;[1 1 1] Bind SendProperty for local users
  (EventDispatchers|BindEventtoCavrnusLaserTargetSpawned (Variables|Default|GetOwner) (delegate Custom|TargetSpawned)))

(event Custom|BindRecieveProperty
  ;[1 1 1] Bind ReceiveProperty from remote users
  (Class|CavrnusFunctionLibrary|BindVectorPropertyValue (Variables|Default|GetSpace%20Connection) (Variables|Default|GetContainerName) "LaserTarget" (delegate Custom|CustomEvent_0)))

(event EventBeginPlay
  ;[0.006856 1 0] Setup - Get specified Laser
  (Class|CavrnusFunctionLibrary|AwaitAnySpaceConnection (delegate Custom|SpaceConnected)))