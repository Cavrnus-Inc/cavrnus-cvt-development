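; Actor component that syncs a pawn's head rotation as a vector property for the Cavrnus integration.
; On BeginPlay it caches the owning BP_BasePawn and its Walk_AnimBP_CVT anim instance, printing a message if the anim cast fails.
; GetVector exposes HeadRotation as a vector.
; SetVector writes incoming values back to the pawn and drives the anim blueprint's HeadLookAt, combined with a fixed 90-degree offset.
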(event EventBeginPlay
  (bind _asbp_base_pawn (Utilities|Casting|CastToBP_BasePawn (Components|GetOwner)))
  (bind _output_get (Variables|Default|SetPawn _asbp_base_pawn))
  (bind _aswalk_anim_bp_cvt (Utilities|Casting|CastToWalk_AnimBP_CVT (Components|SkeletalMesh|GetAnimInstance (Variables|/Script/Engine.Character|GetMesh _output_get)))
    (:then
      (Variables|Default|SetAnim _aswalk_anim_bp_cvt))
    (:CastFailed
      (Development|PrintString "AC_Cavrnus_SyncHead: Casting to WalkAnimBP failed!"))))

(event EventSetVector
  (params (PropertyValue :type Vector :default "0, 0, 0"))
  (bind _pawn (Variables|Default|GetPawn)
    (:then
      (bind _anim (Variables|Default|GetAnim)
        (:then
          (bind _output_get (Variables|/Game/CollaborativeViewer/Blueprints/Pawn/BP_BasePawn.BP_BasePawn_C|SetHeadRotation _pawn (Math|Rotator|MakeRotator (.x PropertyValue) (.y PropertyValue) (.z PropertyValue))))
          (Variables|/Game/CollaborativeViewer/Blueprints/Pawn/Avatar/Animations/Walk_AnimBP_CVT.Walk_AnimBP_CVT_C|SetHeadLookAt _anim (Math|Rotator|CombineRotators "90.000000, 0,90.000000" _output_get)))
        (:else)))
    (:else)))

(fn GetVector
  (bind _pawn (Variables|Default|GetPawn))
  (bind _headrotation (Variables|/Game/CollaborativeViewer/Blueprints/Pawn/BP_BasePawn.BP_BasePawn_C|GetHeadRotation _pawn))
  (return (Math|Vector|MakeVector (.roll _headrotation) (.pitch _headrotation) (.yaw _headrotation))))