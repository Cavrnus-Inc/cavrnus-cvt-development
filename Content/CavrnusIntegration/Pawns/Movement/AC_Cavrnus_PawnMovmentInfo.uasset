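; Actor component in the Cavrnus integration that derives smoothed speed and movement direction for its owning actor.
; Each tick it measures the change in actor location since the previous frame and divides its length by delta time to get raw speed.
; It eases speed with FInterpTo, tuned by acceleration and deceleration values, and lerps the per-frame displacement vector into a smoothed direction using a smoothing factor.
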(event Custom|CalculateSpeed
  (params (DeltaSeconds :type Float%20%28double-precision%29))
  ;[1 1 1] Calculate Speed
  (bind _output_get (Variables|Default|SetCurrentPos (Transformation|GetActorLocation (Variables|Default|GetOwner))))
  (bind _output_get_2 (Variables|Movement|SetMovementDirection (- _output_get (Variables|Default|GetPreviousPos))))
  (bind _output_get_3 (Variables|Default|SetSpeed (/ (Math|Vector|VectorLength _output_get_2) DeltaSeconds)))
  (bind _output_get_4 (Variables|Movement|SetSmoothedSpeed (Math|Interpolation|FInterpTo (Variables|Movement|GetSmoothedSpeed) _output_get_3 (* (Utilities|Time|GetWorldDeltaSeconds) (Variables|Movement|GetDeceleration)) (Variables|Movement|GetAcceleration))))
  (Variables|Default|SetPreviousPos (Variables|Default|GetCurrentPos)))

(event Custom|CalculateSmoothedMovement
  ;[1 1 1] Calculate SmoothedMovement
  (bind _output_get (Variables|Movement|SetSmoothedDirection (Math|Vector|Lerp(Vector) (Variables|Movement|GetSmoothedDirection) (Variables|Movement|GetMovementDirection) (* (Utilities|Time|GetWorldDeltaSeconds) (Variables|Movement|GetSmoothingFactor))))))

(event EventBeginPlay
  ;[0 1 0.01417] BeginPlay
  (Variables|Default|SetOwner (Components|GetOwner)))

(event EventTick
  (params (DeltaSeconds :type Float%20%28single-precision%29))
  ;[0.826 0.2281 0.2194] EventTick
  (Utilities|IsValid (Variables|Default|GetOwner)
    (:Is%20Valid
      (Utilities|FlowControl|Sequence
        (:then_0
          (CallFunction|CalculateSpeed DeltaSeconds))
        (:then_1
          (CallFunction|CalculateSmoothedMovement))))))