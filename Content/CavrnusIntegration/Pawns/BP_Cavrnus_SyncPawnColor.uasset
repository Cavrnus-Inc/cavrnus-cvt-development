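; Pawn component that applies a Cavrnus-synced primary color to its owning BP_BasePawn.
; Once a space connects, it reads the pawn's properties container name and binds to "primaryColor" updates.
; Each update recolors the pawn meshes, player controller color and both lasers, with extra handling for VR pawn controllers and meshes.
; GetColor is an unfinished stub, and the VR-specific right-laser recolor is unwired.
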(event Custom|SpaceConnected
  (params (SpaceConnection :type Cavrnus%20Space%20Connection%20Structure))
  ;[1 0.3401 0.2784] BeginPlay
  (Variables|Default|SetSpace%20Connection SpaceConnection)
  (Utilities|FlowControl|Delay 0.0)
  (Utilities|FlowControl|Sequence
    (:then_0
      (CallFunction|SetupComponents))
    (:then_1
      (CallFunction|SetupBindings))))

(event Custom|SetupComponents
  ;[1 1 1] SetupComponents
  (bind _asbp_base_pawn (Utilities|Casting|CastToBP_BasePawn (Components|GetOwner))
    (:then
      (Variables|Default|SetPawn _asbp_base_pawn)
      (Utilities|IsValid (Actor|GetComponentbyClass (Variables|Default|GetPawn) "/Script/CavrnusConnector.CavrnusPropertiesContainer")
        (:Is%20Valid
          (Variables|Default|SetContainer%20Name (Variables|/Script/CavrnusConnector.CavrnusPropertiesContainer|GetContainerName (Actor|GetComponentbyClass (Variables|Default|GetPawn) "/Script/CavrnusConnector.CavrnusPropertiesContainer"))))))
    (:CastFailed
      (Development|PrintString "SyncPawnColor must exist below a BP_BasePawn."))))

(event Custom|SetupBindings
  ;[1 1 1] SetupBindings
  (Class|CavrnusFunctionLibrary|BindColorPropertyValue (Variables|Default|GetSpace%20Connection) (Variables|Default|GetContainer%20Name) "primaryColor" (delegate Custom|ColorUpdated)))

(event Custom|ColorUpdated
  (params (Value :type Linear%20Color%20Structure) (ContainerName :type String) (PropertyName :type String))
  (bind _pawn (Variables|Default|GetPawn))
  ;[1 1 1] SetupBindings
  (Variables|Default|SetServerColor Value)
  (Utilities|FlowControl|Sequence
    (:then_0
      (bind _output_get (Variables|/Game/CollaborativeViewer/Blueprints/Pawn/BP_BasePawn.BP_BasePawn_C|SetPlayerColor _pawn (Variables|Default|GetServerColor)))
      (CallFunction|ChangeColors (Variables|/Game/CollaborativeViewer/Blueprints/Pawn/BP_BasePawn.BP_BasePawn_C|GetPlayerMeshesArray _pawn) _output_get))
    (:then_1
      (bind _playercontroller (Variables|/Game/CollaborativeViewer/Blueprints/Pawn/BP_BasePawn.BP_BasePawn_C|GetPlayerController (Variables|Default|GetPawn))
        (:then
          (Variables|/Game/CollaborativeViewer/Blueprints/PlayerController/BP_Collab_V_PlayerController.BP_Collab_V_PlayerController_C|SetColor _playercontroller (Variables|Default|GetServerColor)))
        (:else)))
    (:then_2
      (bind _laseractor_r (Variables|/Game/CollaborativeViewer/Blueprints/Pawn/BP_BasePawn.BP_BasePawn_C|GetLaserActor_r (Variables|Default|GetPawn))
        (:then
          (bind _lasermesh (Variables|/Game/CollaborativeViewer/Blueprints/Pawn/Laser.Laser_C|GetLaserMesh _laseractor_r)
            (:then
              (CallFunction|ChangeColors (Utilities|Array|MakeArray _lasermesh) (Variables|Default|GetServerColor)))
            (:else
              (Development|PrintString "Can't change color of Right laser! Not found"))))
        (:else)))
    (:then_3
      (bind _laseractor_l (Variables|/Game/CollaborativeViewer/Blueprints/Pawn/BP_BasePawn.BP_BasePawn_C|GetLaserActor_L (Variables|Default|GetPawn))
        (:then
          (bind _lasermesh_2 (Variables|/Game/CollaborativeViewer/Blueprints/Pawn/Laser.Laser_C|GetLaserMesh _laseractor_l)
            (:then
              (CallFunction|ChangeColors (Utilities|Array|MakeArray _lasermesh_2) (Variables|Default|GetServerColor)))
            (:else
              (Development|PrintString "Can't change color of Left laser! Not found"))))
        (:else)))
    (:then_4
      ;;[0.3941 1 0.9061] Handle VR
      (bind _asbp_vrpawn (Utilities|Casting|CastToBP_VRPawn (Variables|Default|GetPawn)))
      (Variables|/Game/CollaborativeViewer/Blueprints/Pawn/BP_BasePawn.BP_BasePawn_C|SetPlayerColor _asbp_vrpawn (Variables|Default|GetServerColor))
      (Utilities|FlowControl|Sequence
        (:then_0
          (bind _leftcontroller (Variables|/Game/CollaborativeViewer/Blueprints/Pawn/VR/BP_VRPawn.BP_VRPawn_C|GetLeftController _asbp_vrpawn)
            (:then
              (Default|ColorMeshes _leftcontroller))
            (:else)))
        (:then_1
          (bind _rightcontroller (Variables|/Game/CollaborativeViewer/Blueprints/Pawn/VR/BP_VRPawn.BP_VRPawn_C|GetRightController _asbp_vrpawn)
            (:then
              (Default|ColorMeshes _rightcontroller))
            (:else)))
        (:then_2
          (CallFunction|ChangeColors (Variables|/Game/CollaborativeViewer/Blueprints/Pawn/BP_BasePawn.BP_BasePawn_C|GetPlayerMeshesArray _asbp_vrpawn) (Variables|Default|GetServerColor)))
        (:then_3
          (bind _laseractor_l_2 (Variables|/Game/CollaborativeViewer/Blueprints/Pawn/BP_BasePawn.BP_BasePawn_C|GetLaserActor_L _asbp_vrpawn)
            (:then
              (CallFunction|ChangeColors (Utilities|Array|MakeArray (Variables|/Game/CollaborativeViewer/Blueprints/Pawn/Laser.Laser_C|GetLaserMesh _laseractor_l_2)) (Variables|Default|GetServerColor)))
            (:else)))
        (:then_4
          (bind _laseractor_r_2 (Variables|/Game/CollaborativeViewer/Blueprints/Pawn/BP_BasePawn.BP_BasePawn_C|GetLaserActor_r _asbp_vrpawn)
            (:then)
            (:else)))))))

(event EventBeginPlay
  ;[1 0.3401 0.2784] BeginPlay
  (Class|CavrnusFunctionLibrary|AwaitAnySpaceConnection (delegate Custom|SpaceConnected)))

(fn GetColor)