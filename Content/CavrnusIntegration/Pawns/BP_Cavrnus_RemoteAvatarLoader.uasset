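; Represents a remote Cavrnus user by spawning and swapping the avatar pawn that matches that user's movement mode.
; Once a space connection exists, it binds the Movement and AvatarVis properties on its container to drive pawn class and visibility.
; Each swap replaces the pawn at its last transform, passes on the container name and sets up the name tag for the user.
; The spawned avatar is destroyed on EndPlay.
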(event Custom|Connected
  (params (SpaceConnection :type Cavrnus%20Space%20Connection%20Structure))
  (bind _cavrnuspropertiescontainer (Variables|Default|GetCavrnusPropertiesContainer))
  (bind _containername (Variables|/Script/CavrnusConnector.CavrnusPropertiesContainer|GetContainerName _cavrnuspropertiescontainer))
  ;[0.006856 1 0] Wait For Space Connection
  (Variables|Default|SetSpaceConnection SpaceConnection)
  (Utilities|FlowControl|Delay 0.0)
  (if (not (Utilities|Array|IsEmpty _containername))
    (Variables|Default|SetCavrnus%20User (Variables|/Script/CavrnusConnector.CavrnusUserAvatarFlag|GetCavrnusUser (Actor|GetComponentbyClass "/Script/CavrnusConnector.CavrnusUserAvatarFlag")))
    (Class|CavrnusFunctionLibrary|BindStringPropertyValue (Variables|Default|GetSpaceConnection) _containername "Movement" (delegate Custom|MovementUpdated))
    (Class|CavrnusFunctionLibrary|BindBooleanPropertyValue (Variables|Default|GetSpaceConnection) _containername "AvatarVis" (delegate Custom|CustomEvent))))

(event Custom|CustomEvent
  (params (Value :type Boolean) (ContainerName :type String) (PropertyName :type String))
  (bind _currentavatar (Variables|Default|GetCurrentAvatar)
    (:then
      (bind _rootcomponent (Variables|/Script/Engine.Actor|GetRootComponent _currentavatar)
        (:then
          (Rendering|SetVisibility _rootcomponent Value true))
        (:else)))
    (:else)))

(event Custom|MovementUpdated
  (params (Value :type String) (ContainerName :type String) (PropertyName :type String))
  (CallFunction|SwitchMode Value ContainerName))

(event EventBeginPlay
  ;[0.006856 1 0] Wait For Space Connection
  (Class|CavrnusFunctionLibrary|AwaitAnySpaceConnection (delegate Custom|Connected)))

(event EventEndPlay
  (params (EndPlayReason :type EEndPlayReason%20Enum :default "Destroyed"))
  (bind _currentavatar (Variables|Default|GetCurrentAvatar)
    (:then
      (Actor|DestroyActor _currentavatar))
    (:else)))

(fn ConstructionScript)

(fn SwitchMode
  (params (Value :type String) (ContainerName :type String))
  (if (and (Utilities|Enum|NotEqual(Enum) Value (Variables|Default|GetCurrentMode)) (not (Utilities|Array|IsEmpty ContainerName)))
    (bind _output_get (Variables|Default|SetCurrentMode Value))
    (switch string _output_get
      (:Fly
        (CallFunction|SpawnAvatar "/Game/CollaborativeViewer/Blueprints/Pawn/Default/BP_Desktop_FlyMode_Pawn.BP_Desktop_FlyMode_Pawn_C" ContainerName))
      (:Walk
        (CallFunction|SpawnAvatar "/Game/CollaborativeViewer/Blueprints/Pawn/Default/BP_Desktop_WalkMode_Pawn.BP_Desktop_WalkMode_Pawn_C" ContainerName))
      (:Orbit
        (CallFunction|SpawnAvatar "/Game/CollaborativeViewer/Blueprints/Pawn/Default/BP_Desktop_OrbitMode_Pawn.BP_Desktop_OrbitMode_Pawn_C" ContainerName))
      (:VR
        (CallFunction|SpawnAvatar "/Game/CollaborativeViewer/Blueprints/Pawn/VR/BP_VRPawn.BP_VRPawn_C" ContainerName)))))

(fn SpawnAvatar
  (params (AvatarClass :type Actor%20Class%20Reference) (PropertiesContainerName :type String))
  (LocalVariables|SetContainerName PropertiesContainerName)
  (Utilities|IsValid (Variables|Default|GetCurrentAvatar)
    (:Is%20Valid
      (LocalVariables|SetCurrentAvatarTransform (Transformation|GetActorTransform (Variables|Default|GetCurrentAvatar)))
      (Actor|DestroyActor (Variables|Default|GetCurrentAvatar)))
    (:Is%20Not%20Valid
      _))
  (bind _returnvalue (Game|SpawnActorfromClass AvatarClass (LocalVariables|GetCurrentAvatarTransform) "Undefined" "SelectDefaultAtRuntime" 0 0))
  (bind _output_get (Variables|Default|SetCurrentAvatar _returnvalue))
  (if (Utilities|IsValid (Actor|GetComponentbyClass _output_get "/Script/CavrnusConnector.CavrnusPropertiesContainer"))
    (Variables|/Script/CavrnusConnector.CavrnusPropertiesContainer|SetContainerName (Actor|GetComponentbyClass _output_get "/Script/CavrnusConnector.CavrnusPropertiesContainer") (LocalVariables|GetContainerName))
    (CallFunction|SetupNameTag)
    (else
      (Development|PrintString "Didn't find prop container on newly spawned avatar!"))))

(fn SetupNameTag
  (bind _currentavatar (Variables|Default|GetCurrentAvatar)
    (:then
      (bind _asbp_base_pawn (Utilities|Casting|CastToBP_BasePawn _currentavatar))
      (Utilities|IsValid (Variables|/Game/CollaborativeViewer/Blueprints/Pawn/BP_BasePawn.BP_BasePawn_C|GetTextName_W _asbp_base_pawn)
        (:Is%20Valid
          (Utilities|IsValid (UserInterface|GetUserWidgetObject (Variables|/Game/CollaborativeViewer/Blueprints/Pawn/BP_BasePawn.BP_BasePawn_C|GetTextName_W _asbp_base_pawn))
            (:Is%20Valid
              (bind _aswbp_name_tag_widget (Utilities|Casting|CastToWBP_NameTagWidget (UserInterface|GetUserWidgetObject (Variables|/Game/CollaborativeViewer/Blueprints/Pawn/BP_BasePawn.BP_BasePawn_C|GetTextName_W _asbp_base_pawn)))
                (:then
                  (Default|Setup _aswbp_name_tag_widget (Variables|Default|GetCavrnus%20User)))
                (:CastFailed
                  (Development|PrintString "Cast to NameTagWidget failed!"))))))))
    (:else
      (Development|PrintString "Current Avatar is not set!"))))