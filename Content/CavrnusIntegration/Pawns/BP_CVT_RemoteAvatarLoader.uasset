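; Remote avatar loader that spawns and swaps the avatar representing another Cavrnus user in a shared space.
; On space connection it starts in Fly, then binds the user's "Movement" and "AvatarVis" properties to drive mode and visibility.
; Mode changes replace the avatar at its last transform, pass on the properties container name and set up the name tag.
; The spawned avatar is destroyed along with the loader.
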(event Custom|Connected
  (params (SpaceConnection :type Cavrnus%20Space%20Connection%20Structure))
  (bind _cavrnuspropertiescontainer (Variables|Default|GetCavrnusPropertiesContainer))
  (bind _containername (Variables|/Script/CavrnusConnector.CavrnusPropertiesContainer|GetContainerName _cavrnuspropertiescontainer))
  ;[0.006856 1 0] Wait For Space Connection
  (Variables|Default|SetSpaceConnection SpaceConnection)
  (Utilities|FlowControl|Delay 0.0)
  (if (not (Utilities|Array|IsEmpty _containername))
    (Variables|Default|SetCavrnus%20User (Variables|/Script/CavrnusConnector.CavrnusUserAvatarFlag|GetCavrnusUser (Actor|GetComponentbyClass "/Script/CavrnusConnector.CavrnusUserAvatarFlag")))
    (CallFunction|SwitchMode "Fly" _containername)
    (Class|CavrnusFunctionLibrary|BindStringPropertyValue (Variables|Default|GetSpaceConnection) _containername "Movement" (delegate Custom|MovementUpdated))
    (Class|CavrnusFunctionLibrary|BindBooleanPropertyValue (Variables|Default|GetSpaceConnection) (Variables|/Script/CavrnusConnector.CavrnusPropertiesContainer|GetContainerName (Variables|Default|GetCavrnusPropertiesContainer)) "AvatarVis" (delegate Custom|VisUpdated))
    (Game|BindEventtoOnDestroyed (delegate Custom|Destroyed))))

(event Custom|Destroyed
  (params (DestroyedActor :type Actor%20Object%20Reference))
  (bind _currentavatar (Variables|Default|GetCurrentAvatar)
    (:then
      (Actor|DestroyActor _currentavatar))
    (:else)))

(event Custom|MovementUpdated
  (params (Value :type String) (ContainerName :type String) (PropertyName :type String))
  (CallFunction|SwitchMode Value ContainerName)
  (bind _returnvalue (Class|CavrnusFunctionLibrary|GetBoolPropertyValue (Variables|Default|GetSpaceConnection) ContainerName "AvatarVis"))
  (CallFunction|SetAvatarVis _returnvalue))

(event Custom|VisUpdated
  (params (Value :type Boolean) (ContainerName :type String) (PropertyName :type String))
  (CallFunction|SetAvatarVis Value))

(event EventBeginPlay
  ;[0.006856 1 0] Wait For Space Connection
  (Class|CavrnusFunctionLibrary|AwaitAnySpaceConnection (delegate Custom|Connected)))

(event EventEndPlay
  (params (EndPlayReason :type EEndPlayReason%20Enum :default "Destroyed"))
  (bind _currentavatar (Variables|Default|GetCurrentAvatar)
    (:then
      (Actor|DestroyActor _currentavatar))
    (:else)))

(fn ConstructionScript)

(fn SwitchMode
  (params (Value :type String) (ContainerName :type String))
  (if (and (Utilities|Enum|NotEqual(Enum) Value (Variables|Default|GetCurrentMode)) (not (Utilities|Array|IsEmpty ContainerName)))
    (bind _output_get (Variables|Default|SetCurrentMode Value))
    (switch string _output_get
      (:Fly
        (CallFunction|SpawnAvatar "/Game/CavrnusIntegration/Pawns/RemotePawns/BP_CVT_REMOTE_FlyMode.BP_CVT_REMOTE_FlyMode_C" ContainerName))
      (:Walk
        (CallFunction|SpawnAvatar "/Game/CavrnusIntegration/Pawns/RemotePawns/BP_CVT_REMOTE_WalkMode.BP_CVT_REMOTE_WalkMode_C" ContainerName))
      (:VR
        (CallFunction|SpawnAvatar "/Game/CollaborativeViewer/Blueprints/Pawn/VR/BP_VRPawn.BP_VRPawn_C" ContainerName))
      (:Orbit
        (CallFunction|SpawnAvatar "/Game/CavrnusIntegration/Pawns/RemotePawns/BP_CVT_REMOTE_OrbitMode.BP_CVT_REMOTE_OrbitMode_C" ContainerName)))))

(fn SpawnAvatar
  (params (AvatarClass :type Actor%20Class%20Reference) (PropertiesContainerName :type String))
  (if (Utilities|IsValidClass AvatarClass)
    (LocalVariables|SetContainerName PropertiesContainerName)
    (Variables|Default|GetCurrentAvatar
      (:then
        (LocalVariables|SetCurrentAvatarTransform (Transformation|GetActorTransform (Variables|Default|GetCurrentAvatar)))
        (Actor|DestroyActor (Variables|Default|GetCurrentAvatar)))
      (:else
        _))
    (bind _returnvalue (Game|SpawnActorfromClass AvatarClass (LocalVariables|GetCurrentAvatarTransform) "AdjustIfPossibleButAlwaysSpawn" "SelectDefaultAtRuntime" 0 0))
    (bind _output_get (Variables|Default|SetCurrentAvatar _returnvalue))
    (if (Utilities|IsValid (Actor|GetComponentbyClass _output_get "/Script/CavrnusConnector.CavrnusPropertiesContainer"))
      (Variables|/Script/CavrnusConnector.CavrnusPropertiesContainer|SetContainerName (Actor|GetComponentbyClass _output_get "/Script/CavrnusConnector.CavrnusPropertiesContainer") (LocalVariables|GetContainerName))
      (CallFunction|SetupNameTag)
      (else
        (Development|PrintString "Didn't find prop container on newly spawned avatar!")))
    (else
      (Development|PrintString "The avatar class you are trying to spawn is not valid!"))))

(fn SetupNameTag
  (bind _currentavatar (Variables|Default|GetCurrentAvatar)
    (:then
      (if (Utilities|Array|IsNotEmpty (Actor|GetComponentsByClass _currentavatar "/Script/UMG.WidgetComponent"))
        (bind _array_element (Utilities|Array|ForEachLoopwithBreak (Actor|GetComponentsByClass _currentavatar "/Script/UMG.WidgetComponent") :!label _label)
          (:LoopBody
            (Utilities|IsValid (UserInterface|GetUserWidgetObject _array_element)
              (:Is%20Valid
                (goto _label Break))))
          (:Completed
            (bind _aswbp_name_tag_widget (Utilities|Casting|CastToWBP_NameTagWidget (UserInterface|GetUserWidgetObject _array_element)))
            (Default|Setup _aswbp_name_tag_widget (Variables|Default|GetCavrnus%20User))))))
    (:else
      (Development|PrintString "Current Avatar is not set!"))))

(fn SetAvatarVis
  (params (IsVisible :type Boolean))
  (bind _currentavatar (Variables|Default|GetCurrentAvatar)
    (:then
      (bind _rootcomponent (Variables|/Script/Engine.Actor|GetRootComponent _currentavatar)
        (:then
          (Rendering|SetVisibility _rootcomponent IsVisible true))
        (:else)))
    (:else)))