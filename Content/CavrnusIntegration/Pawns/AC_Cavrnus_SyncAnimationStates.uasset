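; Cavrnus component that syncs a BP_BasePawn's animation state (IsInAir and Speed) as a JSON string property.
; After a space connection, it caches the pawn, its properties container name and its Walk_AnimBP instance.
; GetString serializes the anim values, and SetString parses received values back into the AnimBP.
; Tick also overwrites Speed every frame with the pawn movement component's SmoothedSpeed, for smoothed local animation.
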(event Custom|SetupComponents
  (bind _returnvalue (Components|GetOwner))
  ;[0.9697 1 0.9354] SetupComponents
  (bind _asbp_base_pawn (Utilities|Casting|CastToBP_BasePawn _returnvalue)
    (:then
      (Variables|Default|SetPawn _asbp_base_pawn)
      (Variables|Default|SetContainer%20Name (Variables|/Script/CavrnusConnector.CavrnusPropertiesContainer|GetContainerName (Actor|GetComponentbyClass _returnvalue "/Script/CavrnusConnector.CavrnusPropertiesContainer")))
      (bind _aswalk_anim_bp (Utilities|Casting|CastToWalk_AnimBP (Components|SkeletalMesh|GetAnimInstance (Variables|/Script/Engine.Character|GetMesh _asbp_base_pawn)))
        (:then
          (Variables|Default|SetAnimationController _aswalk_anim_bp))
        (:CastFailed
          (Development|PrintString "AnimationBP_Cast Failed!" true true "(R=1.000000,G=0.000000,B=0.138585,A=1.000000)"))))
    (:CastFailed
      (Development|PrintString "SyncAnimationState_Pawn Cast Failed!" true true "(R=1.000000,G=0.000000,B=0.021217,A=1.000000)"))))

(event Custom|SC
  (params (SpaceConnection :type Cavrnus%20Space%20Connection%20Structure))
  ;[1 0.3277 0.3935] BeginPlay
  (Variables|Default|SetSpace%20Connection SpaceConnection)
  (Utilities|FlowControl|Delay 0.0)
  (CallFunction|SetupComponents))

(event EventSetString
  (params (PropertyValue :type String))
  ;[0 1 0.01417] Server Update Value
  (CallFunction|HandleAnimationStateUpdate PropertyValue))

(event EventTick
  (params (DeltaSeconds :type Float%20%28single-precision%29))
  ;[0.9278 0.9317 1] Apply Smoothed Movement Locally
  (bind _pawn (Variables|Default|GetPawn)
    (:then
      (bind _ac_cavrnus_pawnmovmentinfo (Variables|/Game/CollaborativeViewer/Blueprints/Pawn/BP_BasePawn.BP_BasePawn_C|GetAC_Cavrnus_PawnMovmentInfo _pawn)
        (:then
          (bind _animationcontroller (Variables|Default|GetAnimationController)
            (:then
              (Variables|/Game/CollaborativeViewer/Blueprints/Pawn/Avatar/Animations/Walk_AnimBP.Walk_AnimBP_C|SetSpeed _animationcontroller (Variables|/Game/CavrnusIntegration/Pawns/AC_Cavrnus_PawnMovmentInfo.AC_Cavrnus_PawnMovmentInfo_C|GetSmoothedSpeed _ac_cavrnus_pawnmovmentinfo)))
            (:else)))
        (:else)))
    (:else)))

(event EventBeginPlay
  ;[1 0.3277 0.3935] BeginPlay
  (Class|CavrnusFunctionLibrary|AwaitAnySpaceConnection (delegate Custom|SC)))

(fn HandleAnimationStateUpdate
  (params (JsonString :type String))
  (bind _animationcontroller (Variables|Default|GetAnimationController))
  (Utilities|IsValid (Variables|Default|GetAnimationController)
    (:Is%20Valid
      (bind (_outjsonobject _returnvalue) (Class|JsonBlueprintFunctionLibrary|FromString JsonString))
      (if _returnvalue
        (Utilities|FlowControl|Sequence
          (:then_0
            (bind (_outvalue _returnvalue_2) (|GetJsonField _outjsonobject "IsInAir"))
            (if _returnvalue_2
              (Variables|Default|SetIsInAir _outvalue)))
          (:then_1
            (bind (_outvalue_2 _returnvalue_3) (|GetJsonField _outjsonobject "Speed"))
            (if _returnvalue_3
              (Variables|Default|SetSpeed _outvalue_2)))
          (:then_2
            (Utilities|FlowControl|Sequence
              (:then_0
                (Variables|/Game/CollaborativeViewer/Blueprints/Pawn/Avatar/Animations/Walk_AnimBP.Walk_AnimBP_C|SetIsInAir? _animationcontroller (Variables|Default|GetIsInAir)))
              (:then_1
                (Variables|/Game/CollaborativeViewer/Blueprints/Pawn/Avatar/Animations/Walk_AnimBP.Walk_AnimBP_C|SetSpeed _animationcontroller (Variables|Default|GetSpeed))))))))))

(fn GetString
  (bind _animationcontroller (Variables|Default|GetAnimationController))
  (Utilities|IsValid _animationcontroller
    (:Is%20Valid
      (bind _output_get (Variables|Default|SetData (Utilities|Struct|MakeJsonObjectWrapper)))
      (|SetJsonField _output_get "IsInAir" (Variables|/Game/CollaborativeViewer/Blueprints/Pawn/Avatar/Animations/Walk_AnimBP.Walk_AnimBP_C|GetIsInAir? _animationcontroller))
      (|SetJsonField _output_get "Speed" (Variables|/Game/CollaborativeViewer/Blueprints/Pawn/Avatar/Animations/Walk_AnimBP.Walk_AnimBP_C|GetSpeed _animationcontroller))
      (bind _outjsonstring (Class|JsonBlueprintFunctionLibrary|ToString _output_get))
      (return _outjsonstring))))