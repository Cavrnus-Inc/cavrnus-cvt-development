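; Actor component that shares newly created save games with a Cavrnus collaboration space.
; Once connected to a space, it caches pawn and controller references and, for a locally controlled owner, binds to the persistent UI's saving event.
; On save, it polls until the .sav file exists, spawns a saved-game loader object and uploads the file.
; It then posts the uploaded content's ID and name as JSON to that object's SaveFile property.
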(event Custom|OnSpaceConnected
  (params (SpaceConnection :type Cavrnus%20Space%20Connection%20Structure))
  ;[0.03817 1 0.05703] BeginPlay
  (Variables|Default|SetSpaceConnection SpaceConnection)
  (Utilities|FlowControl|Delay 0.0)
  (Utilities|FlowControl|Sequence
    (:then_0
      (CallFunction|GetComponents))
    (:then_1
      (if (Pawn|IsLocallyControlled (Variables|/Script/Engine.Actor|GetInstigator (Components|GetOwner)))
        (CallFunction|SetupBindings)))))

(event Custom|FileUpload
  (params (uploadedContent :type Cavrnus%20Remote%20Content%20Structure%20%28by%20ref%29))
  (bind (_id _name _filename) (Utilities|Struct|BreakCavrnusRemoteContent uploadedContent))
  (bind _jsonobjectwrapper (Utilities|Struct|MakeJsonObjectWrapper))
  ;[1 1 1] SetupBindings
  (Development|PrintString "SaveFileUploaded!" true true "(R=0.000000,G=0.219293,B=1.000000,A=1.000000)" 2e+01)
  (|SetJsonField _jsonobjectwrapper "Id" _id)
  (|SetJsonField _jsonobjectwrapper "Name" _filename)
  (bind (_outjsonstring _returnvalue) (Class|JsonBlueprintFunctionLibrary|ToString _jsonobjectwrapper))
  (if _returnvalue
    (Class|CavrnusFunctionLibrary|PostStringPropertyUpdate (Variables|Default|GetSpaceConnection) (.propertiescontainername (stale Custom|SaveGameCreated _returnvalue)) "SaveFile" _outjsonstring)))

(event Custom|GetComponents
  (bind _returnvalue (Components|GetOwner))
  (bind _returnvalue_2 (Game|GetPlayerController 0))
  (bind _returnvalue_3 (Actor|GetComponentbyClass _returnvalue "/Script/CavrnusConnector.CavrnusPropertiesContainer"))
  ;[1 1 1] GetComponents
  (Utilities|IsValid _returnvalue_3
    (:Is%20Valid
      (Variables|Default|SetContainerName (Variables|/Script/CavrnusConnector.CavrnusPropertiesContainer|GetContainerName _returnvalue_3))
      (bind _asbp_base_pawn (Utilities|Casting|CastToBP_BasePawn (Game|Player|GetPlayerPawn 0)))
      (Variables|Default|SetPawn _asbp_base_pawn)
      (Utilities|IsValid _returnvalue_2
        (:Is%20Valid
          (bind _asbp_collab_v_player_controller (Utilities|Casting|CastToBP_Collab_V_PlayerController _returnvalue_2))
          (Variables|Default|SetPlayerController _asbp_collab_v_player_controller))))))

(event Custom|SetupBindings
  ;[1 1 1] SetupBindings
  (EventDispatchers|BindEventtoSavingState (Variables|/Game/CollaborativeViewer/Blueprints/PlayerController/BP_Collab_V_PlayerController.BP_Collab_V_PlayerController_C|GetPersistent_UI (Variables|Default|GetPlayerController)) (delegate Custom|SaveGameCreated)))

(event Custom|SaveGameCreated
  (params (SlotName :type String%20%28by%20ref%29))
  ;[1 1 1] SetupBindings
  (Development|PrintString "Saving state" true true "(R=0.000000,G=0.660000,B=1.000000,A=1.000000)" 2e+01)
  (bind _output_get (Variables|Default|SetTargetPath (Utilities|String|TrimTrailing (Utilities|String|Append (Class|FilePaths|GetSavedFolder "SaveGames/") (Utilities|String|TrimTrailing SlotName) ".sav"))))
  (if (Class|BlueprintPathsLibrary|FileExists _output_get) :!label _label
    (bind _returnvalue (Class|CavrnusFunctionLibrary|SpawnObject (Variables|Default|GetSpaceConnection) "BP_Cavrnus_SavedGameLoader"))
    (Class|CavrnusFunctionLibrary|UploadContent (Variables|Default|GetTargetPath) (delegate Custom|FileUpload))
    (else
      (Utilities|FlowControl|Delay 0.2)
      (goto _label))))

(event EventBeginPlay
  ;[0.03817 1 0.05703] BeginPlay
  (Class|CavrnusFunctionLibrary|AwaitAnySpaceConnection (delegate Custom|OnSpaceConnected)))