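; Cavrnus save-game receiver that downloads shared save files to the local SaveGames folder and lists them in the player's UI.
; On space connection it caches the container name, pawn and player controller, then binds to the "SaveFile" string property.
; Each non-empty update is parsed as JSON for a content Id, which is fetched to disk.
; The downloaded file's base name is then added to the persistent UI's LoadStateComboBox.
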(event Custom|OnSpaceConnected
  (params (SpaceConnection :type Cavrnus%20Space%20Connection%20Structure))
  ;[0.03817 1 0.05703] BeginPlay
  (Variables|Default|SetSpaceConnection SpaceConnection)
  (Utilities|FlowControl|Delay 0.0)
  (Utilities|FlowControl|Sequence
    (:then_0
      (CallFunction|GetComponents))
    (:then_1
      (CallFunction|SetupBindings))))

(event Custom|GetComponents
  (bind _returnvalue (Game|GetPlayerController 0))
  (bind _returnvalue_2 (Actor|GetComponentbyClass "/Script/CavrnusConnector.CavrnusPropertiesContainer"))
  ;[1 1 1] GetComponents
  (Utilities|IsValid _returnvalue_2
    (:Is%20Valid
      (Variables|Default|SetContainerName (Variables|/Script/CavrnusConnector.CavrnusPropertiesContainer|GetContainerName _returnvalue_2))
      (bind _asbp_base_pawn (Utilities|Casting|CastToBP_BasePawn (Game|Player|GetPlayerPawn 0)))
      (Variables|Default|SetPawn _asbp_base_pawn)
      (Utilities|IsValid _returnvalue
        (:Is%20Valid
          (bind _asbp_collab_v_player_controller (Utilities|Casting|CastToBP_Collab_V_PlayerController _returnvalue))
          (Variables|Default|SetPlayerController _asbp_collab_v_player_controller))))))

(event Custom|GetFileInfo
  (params (StringValue :type String))
  ;[1 1 1] GetFile
  (bind (_outjsonobject _returnvalue) (Class|JsonBlueprintFunctionLibrary|FromString StringValue))
  (if _returnvalue
    (bind _outvalue (|GetJsonField _outjsonobject "Id"))
    (Variables|Default|SetContentId _outvalue)
    (bind _outvalue_2 (|GetJsonField _outjsonobject "Name"))
    (Variables|Default|SetFileName _outvalue_2)
    (Variables|Default|SetSaveLocation (Class|FilePaths|GetSavedFolder "SaveGames/"))))

(event Custom|SetupBindings
  ;[1 1 1] SetupBindings
  (Class|CavrnusFunctionLibrary|BindStringPropertyValue (Variables|Default|GetSpaceConnection) (Variables|Default|GetContainerName) "SaveFile" (delegate Custom|FileIdReceived)))

(event Custom|FileIdReceived
  (params (Value :type String) (ContainerName :type String) (PropertyName :type String))
  ;[1 1 1] SetupBindings
  (if (not (Utilities|Array|IsEmpty Value))
    (Utilities|FlowControl|Sequence
      (:then_0
        (CallFunction|GetFileInfo Value))
      (:then_1
        (CallFunction|SaveFile)))))

(event Custom|SaveFile
  ;[1 1 1] SaveFile
  (Class|CavrnusFunctionLibrary|FetchFilebyIdtoDisk (Variables|Default|GetContentId) (Variables|Default|GetSaveLocation) (delegate Custom|Progress) (delegate Custom|Loaded)))

(event Custom|Progress
  (params (Progress :type Float%20%28single-precision%29) (Step :type String))
  ;[1 1 1] SaveFile
)

(event Custom|Loaded
  (params (fileDest :type String))
  ;[1 1 1] SaveFile
  (bind _output_get (Variables|Default|SetFileName (Class|BlueprintPathsLibrary|GetBaseFilename (Utilities|String|Append "SaveFile loaded at: " fileDest) true)))
  (Default|AddOption (Variables|/Game/CollaborativeViewer/UMG/GameMenu/Persistent_ToolBar.Persistent_ToolBar_C|GetLoadStateComboBox (Variables|/Game/CollaborativeViewer/Blueprints/PlayerController/BP_Collab_V_PlayerController.BP_Collab_V_PlayerController_C|GetPersistent_UI (Variables|Default|GetPlayerController))) _output_get))

(event EventBeginPlay
  ;[0.03817 1 0.05703] BeginPlay
  (Class|CavrnusFunctionLibrary|AwaitAnySpaceConnection (delegate Custom|OnSpaceConnected)))

(fn ConstructionScript)