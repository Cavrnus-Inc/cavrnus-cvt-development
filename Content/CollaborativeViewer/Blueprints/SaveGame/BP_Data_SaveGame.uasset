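; BP_Data_SaveGame is a data Blueprint for the Collaborative Viewer's save game, holding arrays for scene edits and annotations.
; Its arrays cover transformed actors with their transforms and names, X-rayed actors and names, paint annotation points, indices and colors, and text annotations with their locations.
; ClearSaveGameArrays empties all of these arrays in one call, grouped by feature.
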(fn ClearSaveGameArrays
  ;[1 1 1] Transform
  (Utilities|Array|Clear (Variables|TransformCommand|GetTransformedAcrors))
  (Utilities|Array|Clear (Variables|TransformCommand|GetActorTransform))
  (Utilities|Array|Clear (Variables|TransformCommand|GetTransformedObjectNames))
  ;[1 1 1] Xray Actors
  (Utilities|Array|Clear (Variables|XrayCommand|GetXrayActors))
  (Utilities|Array|Clear (Variables|XrayCommand|GetXrayObjectNames))
  ;[1 1 1] Paint Annotation
  (Utilities|Array|Clear (Variables|AnnotationCommand|GetAnnotationPointTransform))
  (Utilities|Array|Clear (Variables|AnnotationCommand|GetAnnotationLastIndex))
  (Utilities|Array|Clear (Variables|AnnotationCommand|GetAnnotationColors))
  ;[1 1 1] Text Annotation
  (Utilities|Array|Clear (Variables|AnnotationCommand|GetAnnotationText))
  (Utilities|Array|Clear (Variables|AnnotationCommand|GetAnnotationTextLocation))
  (Utilities|Array|Clear (Variables|AnnotationCommand|GetAnnotationTargetLocation)))