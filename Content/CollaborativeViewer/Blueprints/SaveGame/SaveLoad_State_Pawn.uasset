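; Collaborative Viewer pawn-side logic that syncs saving, loading and clearing of saved states across connected users.
; Run-on-server (ROS) events relay to multicast (MTC) events that act through the local player controller.
; Saving appends the name and writes the MainSaveGame slot except on dedicated servers; loading only selects the combo box option; clearing empties DataSaveGame arrays.
; Save-time combo box updates are disconnected, noted as handled by Cavrnus bindings.
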(event Custom|LoadSaveGameMTC
  (params (Option :type String))
  (bind _persistent_ui (Variables|Default|GetPersistent_UI)
    (:then
      (Default|SetSelectedOption (Variables|/Game/CollaborativeViewer/UMG/GameMenu/Persistent_ToolBar.Persistent_ToolBar_C|GetLoadStateComboBox _persistent_ui) Option))
    (:else)))

(event Custom|SaveGameMTC
  (params (Option :type String) (SaveGame :type BP%20Name%20Save%20Game%20Object%20Reference))
  (if (not (Networking|IsDedicatedServer))
    (bind _asbp_collab_v_player_controller (Utilities|Casting|CastToBP_Collab_V_PlayerController (Game|GetPlayerController 0)))
    (Utilities|Array|Add (Variables|/Game/CollaborativeViewer/Blueprints/SaveGame/BP_Name_SaveGame.BP_Name_SaveGame_C|GetSaveGameNameArray (Variables|/Game/CollaborativeViewer/Blueprints/SaveGame/SaveLoad_State_Controller.SaveLoad_State_Controller_C|GetSaveGame (Variables|/Game/CollaborativeViewer/Blueprints/PlayerController/BP_Collab_V_PlayerController.BP_Collab_V_PlayerController_C|GetSaveLoad_State_Controller _asbp_collab_v_player_controller))) Option)
    (Utilities|IsValid (Variables|/Game/CollaborativeViewer/Blueprints/SaveGame/SaveLoad_State_Controller.SaveLoad_State_Controller_C|GetSaveGame (Variables|/Game/CollaborativeViewer/Blueprints/PlayerController/BP_Collab_V_PlayerController.BP_Collab_V_PlayerController_C|GetSaveLoad_State_Controller _asbp_collab_v_player_controller))
      (:Is%20Valid
        (SaveGame|SaveGametoSlot (Variables|/Game/CollaborativeViewer/Blueprints/SaveGame/SaveLoad_State_Controller.SaveLoad_State_Controller_C|GetSaveGame (Variables|/Game/CollaborativeViewer/Blueprints/PlayerController/BP_Collab_V_PlayerController.BP_Collab_V_PlayerController_C|GetSaveLoad_State_Controller _asbp_collab_v_player_controller)) "MainSaveGame")))))

(event Custom|LoadSaveGameROS
  (params (Option :type String) (SaveGame :type BP%20Data%20Save%20Game%20Object%20Reference))
  (CallFunction|LoadSaveGameMTC Option))

(event Custom|ClearSaveGamesArraysROS
  (CallFunction|ClearSaveGamesArraysMTC))

(event Custom|ClearSaveGamesArraysMTC
  (bind _asbp_collab_v_player_controller (Utilities|Casting|CastToBP_Collab_V_PlayerController (Game|GetPlayerController 0)))
  (Default|ClearSaveGameArrays (Variables|/Game/CollaborativeViewer/Blueprints/PlayerController/BP_Collab_V_PlayerController.BP_Collab_V_PlayerController_C|GetDataSaveGame _asbp_collab_v_player_controller)))

(event Custom|SaveGameROS
  (params (Option :type String) (SaveGame :type BP%20Name%20Save%20Game%20Object%20Reference))
  (CallFunction|SaveGameMTC Option SaveGame))

(event EventBeginPlay
  (bind _asbp_collab_v_player_controller (Utilities|Casting|CastToBP_Collab_V_PlayerController (Game|GetPlayerController 0)))
  (Variables|Default|SetPersistent_UI (Variables|/Game/CollaborativeViewer/Blueprints/PlayerController/BP_Collab_V_PlayerController.BP_Collab_V_PlayerController_C|GetPersistent_UI _asbp_collab_v_player_controller)))